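; BP_StreetPoles is a construction-script actor that lines a spline with street poles and strings cables between them.
; It adds a static mesh at each spline point, oriented to the spline.
; With NightMode on, each pole gets an emissive dynamic material and a downward spotlight at its "Light" socket.
; Cable components join matching "Cable" sockets on consecutive poles, their lengths randomly shortened from the socket-to-socket distance.
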(fn `UserConstructionScript`
  (bind _spline (`self.Spline`))
  (bind _output (`|GetArrayItem` (`self.StreetPoles`) (+ (`self.Current Loop Index`) 1)))
  (bind _returnvalue_location (`KismetMathLibrary.BreakTransform` (`SceneComponent.GetSocketTransform` _output (`self.CurrentSocketName`) "RTS_World")))
  (bind _returnvalue (`KismetMathLibrary.InverseTransformLocation` (`self.GetTransform` self) _returnvalue_location))
  ;[1 1 1] Set StreetPoles
  (`KismetArrayLibrary.Array_Clear` (`self.StreetPoles`))
  (bind _output_get (set `self.NumberSplinePoints` (- (`SplineComponent.GetNumberOfSplinePoints` _spline) 1)))
  (for _index (range (+ _output_get 1))
    (bind _output_get_2 (set `self.Current Loop Index` _index))
    (bind _returnvalue_2 (`SplineComponent.GetRotationAtSplinePoint` _spline _output_get_2 "Local"))
    (bind _returnvalue_3 (`AddComponent|NODE_AddStaticMeshComponent-0` :`RelativeTransform` (`KismetMathLibrary.MakeTransform` (`SplineComponent.GetLocationAtSplinePoint` _spline _output_get_2 "Local") _returnvalue_2)))
    (`KismetArrayLibrary.Array_Add` (`self.StreetPoles`) _returnvalue_3)
    ;[1 1 1] Add Lights
    (if (`self.Night Mode`)
      (bind _returnvalue_4 (`PrimitiveComponent.CreateDynamicMaterialInstance` _returnvalue_3 0 null "None"))
      (`MaterialInstanceDynamic.SetVectorParameterValue` _returnvalue_4 "Emissive Color" (`self.LightColor`))
      (`MaterialInstanceDynamic.SetScalarParameterValue` _returnvalue_4 "EmissivePower" 200.0)
      (bind _returnvalue_5 (`AddComponent|NODE_AddSpotLightComponent-0` :`RelativeTransform` (`KismetMathLibrary.MakeTransform` (`KismetMathLibrary.InverseTransformLocation` (`self.GetTransform` self) (`SceneComponent.GetSocketLocation` _returnvalue_3 "Light")) (`KismetMathLibrary.MakeRotator` (.roll _returnvalue_2) -90.0 (.yaw _returnvalue_2)))))
      (`LightComponentBase.SetCastShadows` _returnvalue_5 (`self.Cast Shadows?`))
      (`LightComponent.SetLightColor` _returnvalue_5 (`self.LightColor`) true)
      (`LightComponent.SetIntensity` _returnvalue_5 (`self.Light Intensity`))))
  ;[1 1 1] Set Cables
  (for (_array_element _array_index) (`self.StreetPoles`)
    (bind _output_get_3 (set `self.CurrentPole` _array_element))
    (set `self.Current Loop Index` _array_index)
    (for _array_element_2 (`SceneComponent.GetAllSocketNames` _output_get_3)
      (bind _output_get_4 (set `self.CurrentSocketName` _array_element_2))
      (if (`KismetStringLibrary.Contains` (`KismetStringLibrary.Conv_NameToString` _output_get_4) "Cable")
        (`/Engine/EditorBlueprintResources/StandardMacros.IsValid` _output
          (:`Is Valid`
            (bind _returnvalue_location_2 (`KismetMathLibrary.BreakTransform` (`SceneComponent.GetSocketTransform` (`self.CurrentPole`) _output_get_4 "RTS_World")))
            (bind _returnvalue_6 (`KismetMathLibrary.InverseTransformLocation` (`self.GetTransform` self) _returnvalue_location_2))
            (bind _returnvalue_7 (`AddComponent|NODE_AddCableComponent-1` :`RelativeTransform` (`KismetMathLibrary.MakeTransform` _returnvalue_6)))
            (set `CableComponent.CableLength` (- (`KismetMathLibrary.VSize` (- _returnvalue_6 _returnvalue)) (`KismetMathLibrary.RandomFloatInRange` 0.0 400.0)) _returnvalue_7)
            (set `CableComponent.EndLocation` _returnvalue _returnvalue_7)))))))