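; Decal actor for Procedural Russian Apartment Buildings that displays a building number as two digit decals.
; The construction script gives each decal a dynamic material instance and sets its "Number" texture from NumberTex, either randomly or from the two exposed index variables, based on RandomNumber.
; The random first digit starts at index 1, skipping the first texture.
; A random RoughTex entry feeds the "Add Op" parameter to vary opacity.
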(fn `UserConstructionScript`
  (bind _numbertex (`self.NumberTex`))
  (bind _roughtex (`self.RoughTex`))
  (bind _numbertex_2 (`self.NumberTex`))
  (bind _returnvalue (`KismetArrayLibrary.Array_Length` _numbertex))
  (if (`self.Random Number`)
    (`|ExecutionSequence`
      (:`then_0`
        (bind _returnvalue_2 (`DecalComponent.CreateDynamicMaterialInstance` (`self.BuildNum1Decal`)))
        (`MaterialInstanceDynamic.SetTextureParameterValue` _returnvalue_2 "Number" (`|GetArrayItem` _numbertex (`KismetMathLibrary.RandomIntegerInRange` 1 _returnvalue))))
      (:`then_1`
        (bind _returnvalue_3 (`DecalComponent.CreateDynamicMaterialInstance` (`self.BuildNum2Decal`)))
        (`MaterialInstanceDynamic.SetTextureParameterValue` _returnvalue_3 "Number" (`|GetArrayItem` _numbertex (`KismetMathLibrary.RandomIntegerInRange` 0 _returnvalue)))))
    (else
      (`|ExecutionSequence`
        (:`then_0`
          (bind _returnvalue_4 (`DecalComponent.CreateDynamicMaterialInstance` (`self.BuildNum1Decal`)))
          (`MaterialInstanceDynamic.SetTextureParameterValue` _returnvalue_4 "Number" (`|GetArrayItem` _numbertex_2 (`self.Builing Number 1`))))
        (:`then_1`
          (bind _returnvalue_5 (`DecalComponent.CreateDynamicMaterialInstance` (`self.BuildNum2Decal`)))
          (`MaterialInstanceDynamic.SetTextureParameterValue` _returnvalue_5 "Number" (`|GetArrayItem` _numbertex_2 (`self.Builing Number 2`)))))))
  ;[1 1 1] Random Opacity Tex
  (`MaterialInstanceDynamic.SetTextureParameterValue` _returnvalue_3 "Add Op" (`|GetArrayItem` _roughtex (`KismetMathLibrary.RandomIntegerInRange` 0 (`KismetArrayLibrary.Array_Length` _roughtex))))
  (`MaterialInstanceDynamic.SetTextureParameterValue` _returnvalue_2 "Add Op" (`|GetArrayItem` _roughtex (`KismetMathLibrary.RandomIntegerInRange` 0 (`KismetArrayLibrary.Array_Length` _roughtex))))
  (`MaterialInstanceDynamic.SetTextureParameterValue` _returnvalue_4 "Add Op" (`|GetArrayItem` _roughtex (`KismetMathLibrary.RandomIntegerInRange` 0 (`KismetArrayLibrary.Array_Length` _roughtex))))
  (`MaterialInstanceDynamic.SetTextureParameterValue` _returnvalue_5 "Add Op" (`|GetArrayItem` _roughtex (`KismetMathLibrary.RandomIntegerInRange` 0 (`KismetArrayLibrary.Array_Length` _roughtex)))))