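; BP_DamageDecal is a configurable decal actor for placing damage on surfaces, part of the procedural Russian apartment buildings content.
; The construction script creates a dynamic decal material and sets its Mask texture from one of five damage masks chosen by DamageMaskType.
; It also feeds ambient occlusion, tiling and color parameters into that material and toggles a preview plane's visibility.
; The event graph has no active logic.
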(fn `UserConstructionScript`
  (bind _plane (`self.Plane`))
  (bind _decalmatref (`self.DecalMatRef`))
  (`|ExecutionSequence`
    (:`then_0`
      (bind _returnvalue (`DecalComponent.CreateDynamicMaterialInstance` (`self.Decal`)))
      (bind _output_get (set `self.DecalMatRef` _returnvalue))
      (switch `int` (`self.DamageMaskType`)
        (:`1`
          (`MaterialInstanceDynamic.SetTextureParameterValue` _output_get "Mask" "/Game/ProceduralRussianApartmentBuildings/Building_Parts/Mats/Tex/Masks/Damage1_Tex.Damage1_Tex"))
        (:`2`
          (`MaterialInstanceDynamic.SetTextureParameterValue` _output_get "Mask" "/Game/ProceduralRussianApartmentBuildings/Building_Parts/Mats/Tex/Masks/Damage2Mask_Tex.Damage2Mask_Tex"))
        (:`3`
          (`MaterialInstanceDynamic.SetTextureParameterValue` _output_get "Mask" "/Game/ProceduralRussianApartmentBuildings/Building_Parts/Mats/Tex/Masks/Damage3Mask_Tex.Damage3Mask_Tex"))
        (:`4`
          (`MaterialInstanceDynamic.SetTextureParameterValue` _output_get "Mask" "/Game/ProceduralRussianApartmentBuildings/Building_Parts/Mats/Tex/Masks/Damage4Mask_Tex.Damage4Mask_Tex"))
        (:`5`
          (`MaterialInstanceDynamic.SetTextureParameterValue` _output_get "Mask" "/Game/ProceduralRussianApartmentBuildings/Building_Parts/Mats/Tex/Masks/Damage5Mask_Tex.Damage5Mask_Tex"))))
    (:`then_1`
      (`MaterialInstanceDynamic.SetScalarParameterValue` _decalmatref "AO Value" (`self.AO Value`))
      (`MaterialInstanceDynamic.SetScalarParameterValue` _decalmatref "Circuit AO" (`self.Circuit AO`))
      (`MaterialInstanceDynamic.SetScalarParameterValue` _decalmatref "Tile" (`self.Tile`))
      (`MaterialInstanceDynamic.SetVectorParameterValue` _decalmatref "Color" (`self.Color`)))
    (:`then_2`
      (if (`self.PreviewPlane`)
        (`SceneComponent.SetVisibility` _plane true false)
        (else
          (`SceneComponent.SetVisibility` _plane false false))))))