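; BP_BorderSpline is a construction-script tool that lays border meshes along an editable spline.
; It derives the section length from the mesh's X bounds plus a spacing variable, then adds one instance per whole section that fits.
; Each instance follows the spline's local position, pitch and yaw, with slight random sinking and pitch jitter for an uneven look.
; The event graph holds no logic.
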(fn `UserConstructionScript`
  (bind _spline (`self.Spline`))
  (bind _output_get (set `self.SectionLenght` (+ (* (.x (`.BoxExtent` (`KismetMathLibrary.BreakBoxSphereBounds` (`StaticMesh.GetBounds` (`StaticMeshComponent.StaticMesh` (`self.Border`)))))) 2.0) (`self.Distance between`))))
  (for _index (range (`KismetMathLibrary.FTrunc` (/ (`SplineComponent.GetSplineLength` (`self.Spline`)) _output_get)))
    (bind _returnvalue (* _index (`self.SectionLenght`)))
    (bind (_returnvalue_x _returnvalue_y _returnvalue_z) (`KismetMathLibrary.BreakVector` (`SplineComponent.GetLocationAtDistanceAlongSpline` _spline _returnvalue "Local")))
    (bind (_returnvalue_roll _returnvalue_pitch _returnvalue_yaw) (`KismetMathLibrary.BreakRotator` (`SplineComponent.GetRotationAtDistanceAlongSpline` _spline _returnvalue "Local")))
    (`InstancedStaticMeshComponent.AddInstance` (`self.Border`) (`KismetMathLibrary.MakeTransform` (`KismetMathLibrary.MakeVector` _returnvalue_x _returnvalue_y (- _returnvalue_z (`KismetMathLibrary.RandomFloatInRange` 0.0 3.0))) (`KismetMathLibrary.MakeRotator` 0.0 (+ _returnvalue_pitch (`KismetMathLibrary.RandomFloatInRange` -1.0 1.0)) _returnvalue_yaw)))))