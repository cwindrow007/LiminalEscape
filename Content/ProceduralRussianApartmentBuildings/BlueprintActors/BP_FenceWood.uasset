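; BP_FenceWood is a procedural wooden fence actor that builds a row of fence segments in the editor.
; Its construction script creates a dynamic material on the Fence instanced mesh and sets its Color parameter.
; It then adds Segments instances along local X, spaced by the mesh's bounds width plus DistanceBetween.
; The event graph holds no logic.
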(fn `UserConstructionScript`
  (bind _returnvalue (`PrimitiveComponent.CreateDynamicMaterialInstance` (`self.Fence`) 0 null "None"))
  (`MaterialInstanceDynamic.SetVectorParameterValue` _returnvalue "Color" (`self.Color`))
  (for _index (range (`self.Segments`))
    (`InstancedStaticMeshComponent.AddInstance` (`self.Fence`) (`KismetMathLibrary.MakeTransform` (`KismetMathLibrary.MakeVector` (* _index (+ (* (.x (`.BoxExtent` (`KismetMathLibrary.BreakBoxSphereBounds` (`StaticMesh.GetBounds` (`StaticMeshComponent.StaticMesh` (`self.Fence`)))))) 2.0) (`self.Distance between`))))))))