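; BP_FenceMetal is a procedural metal fence actor that builds a straight run of repeated segments in the Construction Script.
; A dynamic material on the Fence component receives the color, damage color and tiling, while DamageType selects one of two damage mask textures.
; Both damage branches then add Segments mesh instances along local X, spaced by mesh bounds width plus DistanceBetween.
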(fn `UserConstructionScript`
  (bind _returnvalue (`PrimitiveComponent.CreateDynamicMaterialInstance` (`self.Fence`) 0 null "None"))
  (`MaterialInstanceDynamic.SetVectorParameterValue` _returnvalue "DamageColor" (`self.Color`))
  (`MaterialInstanceDynamic.SetVectorParameterValue` _returnvalue "Color" (`self.Color2`))
  (`MaterialInstanceDynamic.SetScalarParameterValue` _returnvalue "DamageTile" (`self.Damage Tile`))
  (switch `int` (`self.DamageType`)
    (:`1`
      (`MaterialInstanceDynamic.SetTextureParameterValue` _returnvalue "DamageMask" "/Game/ProceduralRussianApartmentBuildings/Building_Parts/Mats/Tex/Masks/Damage_IN_Alpha_Tex.Damage_IN_Alpha_Tex"))
    (:`2`
      (`MaterialInstanceDynamic.SetTextureParameterValue` _returnvalue "DamageMask" "/Game/ProceduralRussianApartmentBuildings/Building_Parts/Mats/Tex/Masks/Damage0_Mask_Tex.Damage0_Mask_Tex")))
  (for _index (range (`self.Segments`))
    (`InstancedStaticMeshComponent.AddInstance` (`self.Fence`) (`KismetMathLibrary.MakeTransform` (`KismetMathLibrary.MakeVector` (* _index (+ (* (.x (`.BoxExtent` (`KismetMathLibrary.BreakBoxSphereBounds` (`StaticMesh.GetBounds` (`StaticMeshComponent.StaticMesh` (`self.Fence`)))))) 2.0) (`self.Distance between`))))))))