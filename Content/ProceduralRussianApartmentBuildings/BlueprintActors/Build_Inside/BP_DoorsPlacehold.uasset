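; Placeholder actor that lays out stacked doors and jambs inside procedural Russian apartment buildings.
; The construction script adds Jamb instances in a Floors by Row grid, plus one instance each of Door1 and Door2 per floor at a fixed height step.
; Door2 is hidden without collision unless Row exceeds one.
; Left and right door types pick each door component's mesh from DoorsArray using one-based numbering.
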(fn `UserConstructionScript`
  (bind _door2 (`self.Door2`))
  (`|ExecutionSequence`
    (:`then_0`
      (if (not (> (`self.Row`) 1))
        (`SceneComponent.SetVisibility` _door2 false false)
        (`PrimitiveComponent.SetCollisionEnabled` _door2 "NoCollision")))
    (:`then_1`
      (for _index (range (`self.Floors`))
        (for _index_2 (range (`self.Row`))
          (`InstancedStaticMeshComponent.AddInstance` (`self.Jamb`) (`KismetMathLibrary.MakeTransform` (`KismetMathLibrary.MakeVector` (* _index_2 200.0) 0.0 (* _index 250.0))))))
      (for _index_3 (range (`self.Floors`))
        (bind _returnvalue (* _index_3 250.0))
        (`InstancedStaticMeshComponent.AddInstance` (`self.Door1`) (`KismetMathLibrary.MakeTransform` (`KismetMathLibrary.MakeVector` 0.0 0.0 _returnvalue)))
        (`InstancedStaticMeshComponent.AddInstance` (`self.Door2`) (`KismetMathLibrary.MakeTransform` (`KismetMathLibrary.MakeVector` 0.0 0.0 _returnvalue)))))
    (:`then_2`
      (`StaticMeshComponent.SetStaticMesh` (`self.Door1`) (`|GetArrayItem` (`self.DoorsArray`) (- (`self.DoorTypeL`) 1)))
      (`StaticMeshComponent.SetStaticMesh` (`self.Door2`) (`|GetArrayItem` (`self.DoorsArray`) (- (`self.DoorTypeR`) 1))))))