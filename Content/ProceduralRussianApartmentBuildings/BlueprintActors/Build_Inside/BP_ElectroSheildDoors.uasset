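; Interactive electrical panel doors for the apartment building interiors, which the player opens and closes with E.
; A Box trigger enables and disables input on overlap with debug prints, and the key press also checks that the player character is inside.
; An Opened flag plays or reverses one Timeline whose separate tracks swing the right, left and upper doors.
; The construction script tints all three doors through dynamic materials using the Color variable.
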(event `self.Box.OnComponentBeginOverlap`
  (params (OverlappedComponent :type "PrimitiveComponent Object Reference") (OtherActor :type "Actor Object Reference") (OtherComp :type "PrimitiveComponent Object Reference") (OtherBodyIndex :type Integer) (bFromSweep :type Boolean) (SweepResult :type "HitResult Structure (by ref)"))
  (`self.EnableInput` (`GameplayStatics.GetPlayerController` 0))
  (`KismetSystemLibrary.PrintString` "IN RANGE" true true (struct :`R` 0.17682 :`G` 1.0 :`B` 0.474261 :`A` 1.0)))

(event `self.Box.OnComponentEndOverlap`
  (params (OverlappedComponent :type "PrimitiveComponent Object Reference") (OtherActor :type "Actor Object Reference") (OtherComp :type "PrimitiveComponent Object Reference") (OtherBodyIndex :type Integer))
  (`self.DisableInput` (`GameplayStatics.GetPlayerController` 0))
  (`KismetSystemLibrary.PrintString` "NOT IN RANGE" true true (struct :`R` 0.17682 :`G` 1.0 :`B` 0.474261 :`A` 1.0)))

(event `Key|E`
  (params (Key :type "Key Structure"))
  (:`Pressed`
    (if (`PrimitiveComponent.IsOverlappingActor` (`self.Box`) (`GameplayStatics.GetPlayerCharacter` 0))
      (if (`self.Opened?`)
        (set `self.Opened?` false)
        (bind (_direction _r _l _up) (`Timeline|Timeline` :!via `Reverse` :!label _label)
          (:`Update`
            (`SceneComponent.K2_SetRelativeRotation` (`self.DoorR`) (`KismetMathLibrary.RLerp` (struct) (struct :`Yaw` -150.0) _r) false false)
            (`SceneComponent.K2_SetRelativeRotation` (`self.DoorL`) (`KismetMathLibrary.RLerp` (struct) (struct :`Yaw` 140.0) _l) false false)
            (`SceneComponent.K2_SetRelativeRotation` (`self.DoorUP`) (`KismetMathLibrary.RLerp` (struct :`Yaw` 180.0 :`Roll` -180.0) (struct :`Yaw` 180.0 :`Roll` -70.0) _up) false false)))
        (else
          (set `self.Opened?` true)
          (goto _label))))))

(fn `UserConstructionScript`
  ;[1 1 1] Set Color
  (bind _returnvalue (`PrimitiveComponent.CreateDynamicMaterialInstance` (`self.DoorUP`) 0 null "None"))
  (bind _returnvalue_2 (`PrimitiveComponent.CreateDynamicMaterialInstance` (`self.DoorR`) 0 null "None"))
  (bind _returnvalue_3 (`PrimitiveComponent.CreateDynamicMaterialInstance` (`self.DoorL`) 0 null "None"))
  (`MaterialInstanceDynamic.SetVectorParameterValue` _returnvalue_3 "Color" (`self.Color`))
  (`MaterialInstanceDynamic.SetVectorParameterValue` _returnvalue_2 "Color" (`self.Color`))
  (`MaterialInstanceDynamic.SetVectorParameterValue` _returnvalue "Color" (`self.Color`)))