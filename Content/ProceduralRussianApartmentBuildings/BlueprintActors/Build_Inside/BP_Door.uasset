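; BP_Door is a configurable, openable apartment door for the procedural Russian apartment buildings.
; The construction script picks the door mesh by type, shows and positions handles for certain types, and sets jamb width, material and tint colours through dynamic material instances.
; Box overlap enables input when the door can be opened.
; Pressing E inside it plays or reverses a timeline that rotates door and handles, with debug range messages printed.
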(event `self.Box.OnComponentBeginOverlap`
  (params (OverlappedComponent :type "PrimitiveComponent Object Reference") (OtherActor :type "Actor Object Reference") (OtherComp :type "PrimitiveComponent Object Reference") (OtherBodyIndex :type Integer) (bFromSweep :type Boolean) (SweepResult :type "HitResult Structure (by ref)"))
  (if (`self.Can Be Opened?`)
    (`self.EnableInput` (`GameplayStatics.GetPlayerController` 0))
    (`KismetSystemLibrary.PrintString` "IN RANGE" true true (struct :`R` 0.17682 :`G` 1.0 :`B` 0.474261 :`A` 1.0))))

(event `self.Box.OnComponentEndOverlap`
  (params (OverlappedComponent :type "PrimitiveComponent Object Reference") (OtherActor :type "Actor Object Reference") (OtherComp :type "PrimitiveComponent Object Reference") (OtherBodyIndex :type Integer))
  (`self.DisableInput` (`GameplayStatics.GetPlayerController` 0))
  (`KismetSystemLibrary.PrintString` "NOT IN RANGE" true true (struct :`R` 0.17682 :`G` 1.0 :`B` 0.474261 :`A` 1.0)))

(event `Key|E`
  (params (Key :type "Key Structure"))
  (:`Pressed`
    (if (`PrimitiveComponent.IsOverlappingActor` (`self.Box`) (`GameplayStatics.GetPlayerCharacter` 0))
      (if (`self.Opened?`)
        (set `self.Opened?` false)
        (bind (_direction _handle_alpha _window_alpha) (`Timeline|Timeline_0` :!via `Reverse` :!label _label)
          (:`Update`
            (`SceneComponent.K2_SetRelativeRotation` (`self.Handle`) (`KismetMathLibrary.RLerp` (struct) (struct :`Pitch` -55.0) _handle_alpha) false false)
            (`SceneComponent.K2_SetRelativeRotation` (`self.Handle1`) (`KismetMathLibrary.RLerp` (struct :`Roll` 180.0) (struct :`Pitch` -55.0 :`Roll` 180.0) _handle_alpha) false false)
            (`SceneComponent.K2_SetRelativeRotation` (`self.Door`) (`KismetMathLibrary.RLerp` (struct) (struct :`Yaw` -95.0) _window_alpha) false false)))
        (else
          (set `self.Opened?` true)
          (goto _label))))))

(fn `UserConstructionScript`
  (bind _jamb (`self.Jamb`))
  (bind _colorjamb (`self.ColorJamb`))
  (bind _door (`self.Door`))
  (bind (_relativelocation_x _relativelocation_y) (`KismetMathLibrary.BreakVector` (`SceneComponent.RelativeLocation` _door)))
  (`|ExecutionSequence`
    (:`then_0`
      ;[1 1 1] Set Door
      (`StaticMeshComponent.SetStaticMesh` (`self.Door`) (`|GetArrayItem` (`self.Doors`) (`self.DoorType`))))
    (:`then_1`
      ;[1 1 1] Set Knob
      (`self.Set Knob`))
    (:`then_2`
      (if (`self.Wide?`)
        (`StaticMeshComponent.SetStaticMesh` (`self.Jamb`) "/Game/ProceduralRussianApartmentBuildings/Building_Parts/Inside/SM_DoorjambWide.SM_DoorjambWide")
        (`SceneComponent.K2_SetRelativeLocation` _door (`KismetMathLibrary.MakeVector` _relativelocation_x _relativelocation_y 23.0) false false)))
    (:`then_3`
      (if (`self.Iron Jamb?`)
        (`PrimitiveComponent.SetMaterial` _jamb 0 "/Game/ProceduralRussianApartmentBuildings/Building_Parts/Mats/IronDoorjamb_Inst.IronDoorjamb_Inst")
        (else
          (`PrimitiveComponent.SetMaterial` _jamb 0 "/Game/ProceduralRussianApartmentBuildings/Building_Parts/Mats/Rooms/walls/Doorjamb_Plinth_Inst.Doorjamb_Plinth_Inst"))))
    (:`then_4`
      ;[1 1 1] Set Colors
      (bind _returnvalue (`PrimitiveComponent.CreateDynamicMaterialInstance` (`self.Door`) 0 null "None"))
      (bind _returnvalue_2 (`PrimitiveComponent.CreateDynamicMaterialInstance` (`self.Jamb`) 0 null "None"))
      (`MaterialInstanceDynamic.SetVectorParameterValue` _returnvalue_2 "Doorjamb" _colorjamb)
      (`MaterialInstanceDynamic.SetVectorParameterValue` _returnvalue_2 "Color2" _colorjamb)
      (`MaterialInstanceDynamic.SetVectorParameterValue` _returnvalue "C" (`self.DoorTint`)))))