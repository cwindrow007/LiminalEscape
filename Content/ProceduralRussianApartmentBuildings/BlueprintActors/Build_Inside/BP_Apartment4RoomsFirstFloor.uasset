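; Configurable first-floor four-room apartment interior for procedural Russian apartment buildings, assembled in the Construction Script.
; Per-room functions pick wall, ceiling and floor materials by 1-based index on Apartment mesh slots, using dynamic instances for wall colours, tiling and floor rotation.
; Corner adds a child actor when enabled, otherwise swaps to the three-room mesh and disables one radiator.
; Add Balcony spawns one of six variants but is not called here.
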(fn `UserConstructionScript`
  (`|ExecutionSequence`
    (:`then_0`
      (`self.SetCorridor`))
    (:`then_1`
      (`self.SetKitchen`))
    (:`then_2`
      (`self.SetRoomMiddle`))
    (:`then_3`
      (`self.SetBigRoom`))
    (:`then_4`
      (`self.Side Room`))
    (:`then_5`
      (`self.Corner`))))