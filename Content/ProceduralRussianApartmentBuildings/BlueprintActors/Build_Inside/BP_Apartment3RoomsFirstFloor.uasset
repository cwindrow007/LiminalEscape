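; Configurable first-floor three-room apartment interior for procedural Russian apartment buildings, assembled entirely in the construction script.
; Per-room functions style corridor, kitchen, middle and big rooms, picking wall, ceiling and floor materials by one-based index into arrays.
; Dynamic material instances apply wall colors, tiling and floor rotation.
; The Corner flag adds a child actor; otherwise, the mesh becomes the two-room variant and one big-room radiator is disabled.
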(fn `UserConstructionScript`
  (bind _batteryroombig2 (`self.BatteryRoomBig2`))
  (`|ExecutionSequence`
    (:`then_0`
      (`self.SetCorridor`))
    (:`then_1`
      (`self.SetKitchen`))
    (:`then_2`
      (`self.SetRoomMiddle`))
    (:`then_3`
      (`self.SetBigRoom`))
    (:`then_4`
      (if (`self.Corner?`)
        (`AddComponent|NODE_AddChildActorComponent-0` :`RelativeTransform` (`KismetMathLibrary.MakeTransform` (-919.5 -462.299988 -1.6) (struct :`Yaw` 90.0)))
        (else
          (`StaticMeshComponent.SetStaticMesh` (`self.Apartment`) "/Game/ProceduralRussianApartmentBuildings/Building_Parts/Inside/SM_Apart2Rooms1F.SM_Apart2Rooms1F")
          (`SceneComponent.SetVisibility` _batteryroombig2 false false)
          (`PrimitiveComponent.SetCollisionEnabled` _batteryroombig2 "NoCollision"))))))