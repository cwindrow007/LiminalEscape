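; BP_DoorEntrance is an entrance door for procedural Russian apartment buildings that the player toggles open or closed with E.
; A Box overlap enables player input when CanBeOpened is set and disables it on exit, printing debug range messages.
; Pressing E inside the Box flips Opened and plays or reverses a Timeline that lerps the Door's rotation.
; The construction script tints the door through a dynamic material instance using DoorTint.
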(event `self.Box.OnComponentBeginOverlap`
  (params (OverlappedComponent :type "PrimitiveComponent Object Reference") (OtherActor :type "Actor Object Reference") (OtherComp :type "PrimitiveComponent Object Reference") (OtherBodyIndex :type Integer) (bFromSweep :type Boolean) (SweepResult :type "HitResult Structure (by ref)"))
  (if (`self.Can Be Opened?`)
    (`self.EnableInput` (`GameplayStatics.GetPlayerController` 0))
    (`KismetSystemLibrary.PrintString` "IN RANGE" true true (struct :`R` 0.17682 :`G` 1.0 :`B` 0.474261 :`A` 1.0))))

(event `self.Box.OnComponentEndOverlap`
  (params (OverlappedComponent :type "PrimitiveComponent Object Reference") (OtherActor :type "Actor Object Reference") (OtherComp :type "PrimitiveComponent Object Reference") (OtherBodyIndex :type Integer))
  (`self.DisableInput` (`GameplayStatics.GetPlayerController` 0))
  (`KismetSystemLibrary.PrintString` "NOT IN RANGE" true true (struct :`R` 0.17682 :`G` 1.0 :`B` 0.474261 :`A` 1.0)))

(event `Key|E`
  (params (Key :type "Key Structure"))
  (:`Pressed`
    (if (`PrimitiveComponent.IsOverlappingActor` (`self.Box`) (`GameplayStatics.GetPlayerCharacter` 0))
      (if (`self.Opened?`)
        (set `self.Opened?` false)
        (bind (_direction _window_alpha) (`Timeline|Timeline_0` :!via `Reverse` :!label _label)
          (:`Update`
            (`SceneComponent.K2_SetRelativeRotation` (`self.Door`) (`KismetMathLibrary.RLerp` (struct :`Yaw` 180.0) (struct :`Yaw` 60.0) _window_alpha) false false)))
        (else
          (set `self.Opened?` true)
          (goto _label))))))

(fn `UserConstructionScript`
  ;[1 1 1] Set Colors
  (bind _returnvalue (`PrimitiveComponent.CreateDynamicMaterialInstance` (`self.Door`) 0 null "None"))
  (`MaterialInstanceDynamic.SetVectorParameterValue` _returnvalue "MainColor" (`self.DoorTint`)))