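; Procedural three-room apartment interior for Russian apartment buildings, configured entirely in the Construction Script.
; Per-room functions apply indexed wall, ceiling and floor materials to Apartment mesh slots, using dynamic instances for wall colors, tiling and floor rotation.
; The Corner flag adds a child actor; otherwise the mesh becomes SM_Apart2Rooms and the second big-room radiator is hidden without collision.
; BalconyType selects one of six balcony child-actor or static-mesh components.
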(fn `UserConstructionScript`
  (`|ExecutionSequence`
    (:`then_0`
      (`self.SetCorridor`))
    (:`then_1`
      (`self.SetKitchen`))
    (:`then_2`
      (`self.SetRoomMiddle`))
    (:`then_3`
      (`self.SetBigRoom`))
    (:`then_4`
      (`self.Corner`))
    (:`then_5`
      (`self.Add Balcony`))))