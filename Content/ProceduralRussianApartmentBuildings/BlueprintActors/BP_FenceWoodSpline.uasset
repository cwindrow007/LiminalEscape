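; Procedural wooden fence actor that lays instanced fence sections along an editable spline, built entirely in the Construction Script.
; Section spacing comes from the Fence mesh's X bounds plus DistanceBetween, and only as many whole sections as fit the spline length are added.
; Each instance takes the spline's local location and rotation at its distance, at unit scale.
; A dynamic material on the mesh's first slot applies the Color parameter.
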(fn `UserConstructionScript`
  (bind _spline (`self.Spline`))
  (bind _fence (`self.Fence`))
  (bind _returnvalue (`PrimitiveComponent.CreateDynamicMaterialInstance` _fence 0 null "None"))
  (`MaterialInstanceDynamic.SetVectorParameterValue` _returnvalue "Color" (`self.Color`))
  (bind _output_get (set `self.SectionLenght` (+ (* (.x (`.BoxExtent` (`KismetMathLibrary.BreakBoxSphereBounds` (`StaticMesh.GetBounds` (`StaticMeshComponent.StaticMesh` _fence))))) 2.0) (`self.Distance between`))))
  (for _index (range (`KismetMathLibrary.FTrunc` (/ (`SplineComponent.GetSplineLength` (`self.Spline`)) _output_get)))
    (bind _returnvalue_2 (* _index (`self.SectionLenght`)))
    (`InstancedStaticMeshComponent.AddInstance` (`self.Fence`) (`KismetMathLibrary.MakeTransform` (`SplineComponent.GetLocationAtDistanceAlongSpline` _spline _returnvalue_2 "Local") (`SplineComponent.GetRotationAtDistanceAlongSpline` _spline _returnvalue_2 "Local")))))