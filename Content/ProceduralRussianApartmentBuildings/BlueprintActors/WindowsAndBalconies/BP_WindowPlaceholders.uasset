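; Procedural apartment-building facade actor that builds windows, balconies and fake room interiors entirely in the Construction Script.
; Segment and floor counts drive instanced fake rooms and side windows, with an optional first floor and front windows either instanced or randomly picked per component.
; Room material slots get random apartment sets, with dynamic materials varying curtains and applying emissive settings.
; LeftSide and RightSide toggles hide that side's windows and room materials.
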(fn `UserConstructionScript`
  (bind _winsidel1 (`self.WinSideL1`))
  (bind _winsider2 (`self.WinSideR2`))
  (bind _fakerooms (`self.FakeRooms`))
  (bind _fakeroomsff (`self.FakeRoomsFF`))
  (bind _fakerooms_2 (`self.FakeRooms`))
  (`|ExecutionSequence`
    (:`then_0`
      (`self.Create Fake Rooms and Windows`))
    (:`then_1`
      (`self.Randomize fake appartments ` (`self.FakeRoomsFF`)))
    (:`then_2`
      (`self.Randomize fake appartments ` (`self.FakeRooms`)))
    (:`then_3`
      (if (not (`self.LeftSide`))
        (`PrimitiveComponent.SetMaterial` _fakerooms_2 14 "/Game/ProceduralRussianApartmentBuildings/Building_Parts/Mats/FakeRooms/Invisible_M.Invisible_M")
        (`PrimitiveComponent.SetMaterial` (`self.FakeRoomsFF`) 14 "/Game/ProceduralRussianApartmentBuildings/Building_Parts/Mats/FakeRooms/Invisible_M.Invisible_M")
        (`PrimitiveComponent.SetMaterial` (`self.FakeRoomsFF`) 15 "/Game/ProceduralRussianApartmentBuildings/Building_Parts/Mats/FakeRooms/Invisible_M.Invisible_M")
        (`PrimitiveComponent.SetMaterial` _fakerooms_2 15 "/Game/ProceduralRussianApartmentBuildings/Building_Parts/Mats/FakeRooms/Invisible_M.Invisible_M")
        (`PrimitiveComponent.SetMaterial` _fakerooms_2 18 "/Game/ProceduralRussianApartmentBuildings/Building_Parts/Mats/FakeRooms/Invisible_M.Invisible_M")
        (`PrimitiveComponent.SetMaterial` (`self.FakeRoomsFF`) 18 "/Game/ProceduralRussianApartmentBuildings/Building_Parts/Mats/FakeRooms/Invisible_M.Invisible_M")
        (`PrimitiveComponent.SetMaterial` _fakerooms_2 21 "/Game/ProceduralRussianApartmentBuildings/Building_Parts/Mats/FakeRooms/Invisible_M.Invisible_M")
        (`PrimitiveComponent.SetMaterial` (`self.FakeRoomsFF`) 21 "/Game/ProceduralRussianApartmentBuildings/Building_Parts/Mats/FakeRooms/Invisible_M.Invisible_M")
        (`SceneComponent.SetVisibility` _winsidel1 false false)
        (`SceneComponent.SetVisibility` (`self.WinSideL2`) false false)
        (`SceneComponent.SetVisibility` (`self.WinSideL1FF`) false false)
        (`SceneComponent.SetVisibility` (`self.WinSideL2FF`) false false)
        (`PrimitiveComponent.SetCollisionEnabled` _winsidel1 "NoCollision")
        (`PrimitiveComponent.SetCollisionEnabled` (`self.WinSideL2`) "NoCollision")
        (`PrimitiveComponent.SetCollisionEnabled` (`self.WinSideL1FF`) "NoCollision")
        (`PrimitiveComponent.SetCollisionEnabled` (`self.WinSideL2FF`) "NoCollision"))
      (if (not (`self.RightSide`))
        (`PrimitiveComponent.SetMaterial` _fakerooms 16 "/Game/ProceduralRussianApartmentBuildings/Building_Parts/Mats/FakeRooms/Invisible_M.Invisible_M")
        (`PrimitiveComponent.SetMaterial` _fakeroomsff 16 "/Game/ProceduralRussianApartmentBuildings/Building_Parts/Mats/FakeRooms/Invisible_M.Invisible_M")
        (`PrimitiveComponent.SetMaterial` _fakeroomsff 17 "/Game/ProceduralRussianApartmentBuildings/Building_Parts/Mats/FakeRooms/Invisible_M.Invisible_M")
        (`PrimitiveComponent.SetMaterial` _fakerooms 17 "/Game/ProceduralRussianApartmentBuildings/Building_Parts/Mats/FakeRooms/Invisible_M.Invisible_M")
        (`PrimitiveComponent.SetMaterial` _fakerooms 19 "/Game/ProceduralRussianApartmentBuildings/Building_Parts/Mats/FakeRooms/Invisible_M.Invisible_M")
        (`PrimitiveComponent.SetMaterial` _fakeroomsff 19 "/Game/ProceduralRussianApartmentBuildings/Building_Parts/Mats/FakeRooms/Invisible_M.Invisible_M")
        (`PrimitiveComponent.SetMaterial` _fakeroomsff 22 "/Game/ProceduralRussianApartmentBuildings/Building_Parts/Mats/FakeRooms/Invisible_M.Invisible_M")
        (`PrimitiveComponent.SetMaterial` _fakerooms 22 "/Game/ProceduralRussianApartmentBuildings/Building_Parts/Mats/FakeRooms/Invisible_M.Invisible_M")
        (`SceneComponent.SetVisibility` _winsider2 false false)
        (`SceneComponent.SetVisibility` (`self.WinSideR1`) false false)
        (`SceneComponent.SetVisibility` (`self.WinSideR2FF`) false false)
        (`SceneComponent.SetVisibility` (`self.WinSideR1FF`) false false)
        (`PrimitiveComponent.SetCollisionEnabled` _winsider2 "NoCollision")
        (`PrimitiveComponent.SetCollisionEnabled` (`self.WinSideR1`) "NoCollision")
        (`PrimitiveComponent.SetCollisionEnabled` (`self.WinSideR2FF`) "NoCollision")
        (`PrimitiveComponent.SetCollisionEnabled` (`self.WinSideR1FF`) "NoCollision")))))