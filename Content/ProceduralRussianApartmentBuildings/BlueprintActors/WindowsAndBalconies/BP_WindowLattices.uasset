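; Window lattice actor for procedural Russian apartment buildings that randomizes a set of long, short and vent lattice components.
; The construction script gives each component a random mesh variant from its category or hides it.
; Long and short lattices also get a dynamic material instance with a random RGB color; vent lattices keep their materials.
; All randomness is unseeded and the event graph is empty, so the look can change whenever construction reruns.
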(fn `UserConstructionScript`
  (bind _returnvalue (`KismetMathLibrary.RandomFloatInRange` 0.0 1.0))
  (bind _returnvalue_2 (`KismetMathLibrary.RandomFloatInRange` 0.0 1.0))
  (for _array_element (`|MakeArray` (`self.LatticeLong5`) (`self.LatticeLong2`) (`self.LatticeLong3`) (`self.LatticeLong4`) (`self.LatticeLong1`) (`self.LatticeLong6`) (`self.LatticeLong7`) (`self.LatticeLong8`) (`self.LatticeLong9`))
    (`SceneComponent.SetVisibility` _array_element true false)
    (bind _returnvalue_3 (`PrimitiveComponent.CreateDynamicMaterialInstance` _array_element 0 null "None"))
    (`MaterialInstanceDynamic.SetVectorParameterValue` _returnvalue_3 "Color" (make `LinearColor` _returnvalue_2 _returnvalue_2 _returnvalue_2 1.0))
    (switch `int` (`KismetMathLibrary.RandomIntegerInRange` 0 5)
      (:`0`
        (`StaticMeshComponent.SetStaticMesh` _array_element "/Game/ProceduralRussianApartmentBuildings/Building_Parts/WindowsAndFakeRooms/SM_WindowLatticeLong1.SM_WindowLatticeLong1"))
      (:`1`
        (`StaticMeshComponent.SetStaticMesh` _array_element "/Game/ProceduralRussianApartmentBuildings/Building_Parts/WindowsAndFakeRooms/SM_WindowLatticeLong2.SM_WindowLatticeLong2"))
      (:`2`
        (`StaticMeshComponent.SetStaticMesh` _array_element "/Game/ProceduralRussianApartmentBuildings/Building_Parts/WindowsAndFakeRooms/SM_WindowLatticeLong3.SM_WindowLatticeLong3"))
      (:`3`
        (`StaticMeshComponent.SetStaticMesh` _array_element "/Game/ProceduralRussianApartmentBuildings/Building_Parts/WindowsAndFakeRooms/SM_WindowLatticeLong4.SM_WindowLatticeLong4"))
      (:`4`
        (`StaticMeshComponent.SetStaticMesh` _array_element "/Game/ProceduralRussianApartmentBuildings/Building_Parts/WindowsAndFakeRooms/SM_WindowLatticeLong5.SM_WindowLatticeLong5"))
      (:`5`
        (`SceneComponent.SetVisibility` _array_element false false))))
  (for _array_element_2 (`|MakeArray` (`self.LatticeShort2`) (`self.LatticeShort3`) (`self.LatticeShort4`) (`self.LatticeShort1`))
    (`SceneComponent.SetVisibility` _array_element_2 true false)
    (bind _returnvalue_4 (`PrimitiveComponent.CreateDynamicMaterialInstance` _array_element_2 0 null "None"))
    (`MaterialInstanceDynamic.SetVectorParameterValue` _returnvalue_4 "Color" (make `LinearColor` _returnvalue _returnvalue _returnvalue 1.0))
    (switch `int` (`KismetMathLibrary.RandomIntegerInRange` 0 7)
      (:`0`
        (`StaticMeshComponent.SetStaticMesh` _array_element_2 "/Game/ProceduralRussianApartmentBuildings/Building_Parts/WindowsAndFakeRooms/SM_WindowLatticeShort1.SM_WindowLatticeShort1"))
      (:`1`
        (`StaticMeshComponent.SetStaticMesh` _array_element_2 "/Game/ProceduralRussianApartmentBuildings/Building_Parts/WindowsAndFakeRooms/SM_WindowLatticeShort2.SM_WindowLatticeShort2"))
      (:`2`
        (`StaticMeshComponent.SetStaticMesh` _array_element_2 "/Game/ProceduralRussianApartmentBuildings/Building_Parts/WindowsAndFakeRooms/SM_WindowLatticeShort3.SM_WindowLatticeShort3"))
      (:`3`
        (`StaticMeshComponent.SetStaticMesh` _array_element_2 "/Game/ProceduralRussianApartmentBuildings/Building_Parts/WindowsAndFakeRooms/SM_WindowLatticeShort4.SM_WindowLatticeShort4"))
      (:`4`
        (`StaticMeshComponent.SetStaticMesh` _array_element_2 "/Game/ProceduralRussianApartmentBuildings/Building_Parts/WindowsAndFakeRooms/SM_WindowLatticeShort4.SM_WindowLatticeShort4"))
      (:`5`
        (`StaticMeshComponent.SetStaticMesh` _array_element_2 "/Game/ProceduralRussianApartmentBuildings/Building_Parts/WindowsAndFakeRooms/SM_WindowLatticeShort5.SM_WindowLatticeShort5"))
      (:`6`
        (`StaticMeshComponent.SetStaticMesh` _array_element_2 "/Game/ProceduralRussianApartmentBuildings/Building_Parts/WindowsAndFakeRooms/SM_WindowLatticeShort6.SM_WindowLatticeShort6"))
      (:`7`
        (`SceneComponent.SetVisibility` _array_element_2 false false))))
  (for _array_element_3 (`|MakeArray` (`self.LatticeVent1`) (`self.LatticeVent2`) (`self.LatticeVent3`) (`self.LatticeVent4`) (`self.LatticeVent5`))
    (`SceneComponent.SetVisibility` _array_element_3 true false)
    (switch `int` (`KismetMathLibrary.RandomIntegerInRange` 0 5)
      (:`0`
        (`StaticMeshComponent.SetStaticMesh` _array_element_3 "/Game/ProceduralRussianApartmentBuildings/Building_Parts/Facade/SM_VentLattice1.SM_VentLattice1"))
      (:`1`
        (`StaticMeshComponent.SetStaticMesh` _array_element_3 "/Game/ProceduralRussianApartmentBuildings/Building_Parts/Facade/SM_VentLattice2.SM_VentLattice2"))
      (:`2`
        (`StaticMeshComponent.SetStaticMesh` _array_element_3 "/Game/ProceduralRussianApartmentBuildings/Building_Parts/Facade/SM_VentLattice3.SM_VentLattice3"))
      (:`3`
        (`StaticMeshComponent.SetStaticMesh` _array_element_3 "/Game/ProceduralRussianApartmentBuildings/Building_Parts/Facade/SM_VentLattice4.SM_VentLattice4"))
      (:`4`
        (`StaticMeshComponent.SetStaticMesh` _array_element_3 "/Game/ProceduralRussianApartmentBuildings/Building_Parts/Facade/SM_VentLattice5.SM_VentLattice5"))
      (:`5`
        (`SceneComponent.SetVisibility` _array_element_3 false false)))))