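; Building facade module for procedural apartment buildings that shows windows with fake room interiors behind them.
; The construction script picks window and room meshes by front or back side, first floor and window type, and hides unused side pieces.
; Set Fake Apartments assigns room materials per left and right apartment type, then wraps them in dynamic instances to apply emissive power and color.
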(fn `UserConstructionScript`
  (bind _sidefaker (`self.SideFakeR`))
  (bind _sidewinl (`self.SideWinL`))
  (`|ExecutionSequence`
    (:`then_0`
      (if (not (`self.Backside?`))
        ;[1 1 1] Front Windows
        (`|ExecutionSequence`
          (:`then_0`
            (if (`self.FirstFloor`)
              (`StaticMeshComponent.SetStaticMesh` (`self.FakeRooms`) "/Game/ProceduralRussianApartmentBuildings/Building_Parts/WindowsAndFakeRooms/SM_FakeRoomsFirstFront.SM_FakeRoomsFirstFront")
              (`SceneComponent.K2_SetRelativeLocation` (`self.Windows`) (0.0 20.0 0.0) false false)))
          (:`then_1`
            (`StaticMeshComponent.SetStaticMesh` (`self.Windows`) (`|GetArrayItem` (`self.WindowsFrontArray`) (- (`self.WindowsType`) 1)))))
        (else
          ;[1 1 1] Back Windows
          (`StaticMeshComponent.SetStaticMesh` (`self.FakeRooms`) "/Game/ProceduralRussianApartmentBuildings/Building_Parts/WindowsAndFakeRooms/SM_FakeRoomsBack.SM_FakeRoomsBack")
          (`|ExecutionSequence`
            (:`then_0`
              (if (`self.FirstFloor`)
                (`StaticMeshComponent.SetStaticMesh` (`self.FakeRooms`) "/Game/ProceduralRussianApartmentBuildings/Building_Parts/WindowsAndFakeRooms/SM_FakeRoomsFirstBack.SM_FakeRoomsFirstBack")
                (`SceneComponent.K2_SetRelativeLocation` (`self.Windows`) (0.0 20.0 0.0) false false)))
            (:`then_1`
              (`StaticMeshComponent.SetStaticMesh` (`self.Windows`) (`|GetArrayItem` (`self.WindowsBackArray`) (- (`self.WindowsType`) 1))))))))
    (:`then_1`
      (if (not (`self.LeftSide`))
        (`SceneComponent.SetVisibility` _sidewinl false false)
        (`SceneComponent.SetVisibility` (`self.SideFakeL`) false false)
        (`PrimitiveComponent.SetCollisionEnabled` _sidewinl "NoCollision")
        (`PrimitiveComponent.SetCollisionEnabled` (`self.SideFakeL`) "NoCollision"))
      (if (not (`self.RightSide`))
        (`SceneComponent.SetVisibility` _sidefaker false false)
        (`SceneComponent.SetVisibility` (`self.SideWinR`) false false)
        (`PrimitiveComponent.SetCollisionEnabled` _sidefaker "NoCollision")
        (`PrimitiveComponent.SetCollisionEnabled` (`self.SideWinR`) "NoCollision")))
    (:`then_2`
      ;[1 1 1] Set Fake Apartments
      (`self.Set Fake Apartments`))))