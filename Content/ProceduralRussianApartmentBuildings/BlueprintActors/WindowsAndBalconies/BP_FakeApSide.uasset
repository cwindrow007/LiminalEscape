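; BP_FakeApSide is a side window piece with a fake room for procedural Russian apartment buildings, configured entirely in the construction script.
; WindowType picks one of three short window meshes, and FakeRoomType picks one of six room material instances for slot 1 of FakeRoomSide.
; That slot then gets a dynamic material instance driven by EmissiveColor and EmissivePower, so each placed piece carries its own room glow.
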(fn `UserConstructionScript`
  (bind _windshort1 (`self.WindShort1`))
  (bind _fakeroomside (`self.FakeRoomSide`))
  (`|ExecutionSequence`
    (:`then_0`
      (switch `int` (- (`self.WindowType`) 1)
        (:`0`
          (`StaticMeshComponent.SetStaticMesh` _windshort1 "/Game/ProceduralRussianApartmentBuildings/Building_Parts/WindowsAndFakeRooms/SM_WindShort1.SM_WindShort1"))
        (:`1`
          (`StaticMeshComponent.SetStaticMesh` _windshort1 "/Game/ProceduralRussianApartmentBuildings/Building_Parts/WindowsAndFakeRooms/SM_WindShort2.SM_WindShort2"))
        (:`2`
          (`StaticMeshComponent.SetStaticMesh` _windshort1 "/Game/ProceduralRussianApartmentBuildings/Building_Parts/WindowsAndFakeRooms/SM_WindShort3.SM_WindShort3"))))
    (:`then_1`
      (switch `int` (- (`self.FakeRoomType`) 1)
        (:`0`
          (`PrimitiveComponent.SetMaterial` _fakeroomside 1 "/Game/ProceduralRussianApartmentBuildings/Building_Parts/Mats/FakeRooms/3Rooms1/3R1_S_Inst.3R1_S_Inst"))
        (:`1`
          (`PrimitiveComponent.SetMaterial` _fakeroomside 1 "/Game/ProceduralRussianApartmentBuildings/Building_Parts/Mats/FakeRooms/3Rooms2/3R2_S_Inst.3R2_S_Inst"))
        (:`2`
          (`PrimitiveComponent.SetMaterial` _fakeroomside 1 "/Game/ProceduralRussianApartmentBuildings/Building_Parts/Mats/FakeRooms/3Rooms3/3R3_S_Inst.3R3_S_Inst"))
        (:`3`
          (`PrimitiveComponent.SetMaterial` _fakeroomside 1 "/Game/ProceduralRussianApartmentBuildings/Building_Parts/Mats/FakeRooms/3Rooms4/3R4_S_Inst.3R4_S_Inst"))
        (:`4`
          (`PrimitiveComponent.SetMaterial` _fakeroomside 1 "/Game/ProceduralRussianApartmentBuildings/Building_Parts/Mats/FakeRooms/4Rooms1/4R1_S_Inst.4R1_S_Inst"))
        (:`5`
          (`PrimitiveComponent.SetMaterial` _fakeroomside 1 "/Game/ProceduralRussianApartmentBuildings/Building_Parts/Mats/FakeRooms/4Rooms2/4R2_S_Inst.4R2_S_Inst")))
      (bind _returnvalue (`PrimitiveComponent.CreateDynamicMaterialInstance` _fakeroomside 1 null "None"))
      (`MaterialInstanceDynamic.SetVectorParameterValue` _returnvalue "EmissiveColor" (`self.EmissiveColor`))
      (`MaterialInstanceDynamic.SetScalarParameterValue` _returnvalue "EmissivePower" (`self.EmissivePower`)))))