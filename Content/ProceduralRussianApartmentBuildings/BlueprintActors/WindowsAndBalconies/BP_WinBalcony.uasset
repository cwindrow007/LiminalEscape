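; Balcony window-and-door actor for the apartment buildings, with a window and a balcony door that the player can open and close independently.
; A box trigger enables input and prints debug range messages; while overlapping, Shift+E toggles the window and E toggles the door.
; Each toggle plays or reverses its own timeline, lerping handle and panel rotations.
; The construction script optionally applies wood frame and iron handle materials via WoodMat.
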(event `self.Box.OnComponentBeginOverlap`
  (params (OverlappedComponent :type "PrimitiveComponent Object Reference") (OtherActor :type "Actor Object Reference") (OtherComp :type "PrimitiveComponent Object Reference") (OtherBodyIndex :type Integer) (bFromSweep :type Boolean) (SweepResult :type "HitResult Structure (by ref)"))
  (`self.EnableInput` (`GameplayStatics.GetPlayerController` 0))
  (`KismetSystemLibrary.PrintString` "IN RANGE" true true (struct :`R` 0.17682 :`G` 1.0 :`B` 0.474261 :`A` 1.0)))

(event `self.Box.OnComponentEndOverlap`
  (params (OverlappedComponent :type "PrimitiveComponent Object Reference") (OtherActor :type "Actor Object Reference") (OtherComp :type "PrimitiveComponent Object Reference") (OtherBodyIndex :type Integer))
  (`self.DisableInput` (`GameplayStatics.GetPlayerController` 0))
  (`KismetSystemLibrary.PrintString` "NOT IN RANGE" true true (struct :`R` 0.17682 :`G` 1.0 :`B` 0.474261 :`A` 1.0)))

(event `Key|Shift+E`
  (params (Key :type "Key Structure"))
  (:`Pressed`
    (if (`PrimitiveComponent.IsOverlappingActor` (`self.Box`) (`GameplayStatics.GetPlayerCharacter` 0))
      (if (`self.Win1Opened?`)
        (set `self.Win1Opened?` false)
        (bind (_direction _handle_alpha _window_alpha) (`Timeline|Timeline` :!via `Reverse` :!label _label)
          (:`Update`
            (`SceneComponent.K2_SetRelativeRotation` (`self.HandleWin`) (`KismetMathLibrary.RLerp` (struct :`Pitch` -90.0) (struct :`Pitch` -180.0) _handle_alpha) false false)
            (`SceneComponent.K2_SetRelativeRotation` (`self.Win`) (`KismetMathLibrary.RLerp` (struct) (struct :`Yaw` -90.0) _window_alpha) false false)))
        (else
          (set `self.Win1Opened?` true)
          (goto _label))))))

(event `Key|E`
  (params (Key :type "Key Structure"))
  (:`Pressed`
    (if (`PrimitiveComponent.IsOverlappingActor` (`self.Box`) (`GameplayStatics.GetPlayerCharacter` 0))
      (if (`self.Win2Opened?`)
        (set `self.Win2Opened?` false)
        (bind (_direction _handle_alpha _window_alpha) (`Timeline|Timeline_0` :!via `Reverse` :!label _label_2)
          (:`Update`
            (`SceneComponent.K2_SetRelativeRotation` (`self.HandleDoor`) (`KismetMathLibrary.RLerp` (struct :`Pitch` -90.0) (struct) _handle_alpha) false false)
            (`SceneComponent.K2_SetRelativeRotation` (`self.HandleDoor1`) (`KismetMathLibrary.RLerp` (struct :`Pitch` -90.0 :`Roll` 180.0) (struct :`Roll` 180.0) _handle_alpha) false false)
            (`SceneComponent.K2_SetRelativeRotation` (`self.BalcDoor`) (`KismetMathLibrary.RLerp` (struct) (struct :`Yaw` 90.0) _window_alpha) false false)))
        (else
          (set `self.Win2Opened?` true)
          (goto _label_2))))))

(fn `UserConstructionScript`
  (if (`self.WoodMat`)
    (`PrimitiveComponent.SetMaterial` (`self.Frame`) 1 "/Game/ProceduralRussianApartmentBuildings/Building_Parts/Mats/Windows/WindowsPacks/WindCombWood_Inst.WindCombWood_Inst")
    (`PrimitiveComponent.SetMaterial` (`self.BalcDoor`) 1 "/Game/ProceduralRussianApartmentBuildings/Building_Parts/Mats/Windows/WindowsPacks/WindCombWood_Inst.WindCombWood_Inst")
    (`PrimitiveComponent.SetMaterial` (`self.Win`) 1 "/Game/ProceduralRussianApartmentBuildings/Building_Parts/Mats/Windows/WindowsPacks/WindCombWood_Inst.WindCombWood_Inst")
    (`PrimitiveComponent.SetMaterial` (`self.HandleDoor`) 0 "/Game/ProceduralRussianApartmentBuildings/Building_Parts/Mats/Windows/Balconies/WinHandleIron_Inst.WinHandleIron_Inst")
    (`PrimitiveComponent.SetMaterial` (`self.HandleWin`) 0 "/Game/ProceduralRussianApartmentBuildings/Building_Parts/Mats/Windows/Balconies/WinHandleIron_Inst.WinHandleIron_Inst")
    (`PrimitiveComponent.SetMaterial` (`self.HandleDoor1`) 0 "/Game/ProceduralRussianApartmentBuildings/Building_Parts/Mats/Windows/Balconies/WinHandleIron_Inst.WinHandleIron_Inst")))