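; BP_BorderStraight is a procedural prop actor that lays out a straight row of border pieces, from the procedural Russian apartment buildings content.
; Its construction script adds one Border mesh instance per segment along local X, stepping by the mesh's bounds length plus DistanceBetween.
; Each instance gets a slight random vertical drop and pitch, unseeded, for an uneven look.
; The event graph holds no active logic.
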(fn `UserConstructionScript`
  (for _index (range (`self.Segments`))
    (`InstancedStaticMeshComponent.AddInstance` (`self.Border`) (`KismetMathLibrary.MakeTransform` (`KismetMathLibrary.MakeVector` (* _index (+ (* (.x (`.BoxExtent` (`KismetMathLibrary.BreakBoxSphereBounds` (`StaticMesh.GetBounds` (`StaticMeshComponent.StaticMesh` (`self.Border`)))))) 2.0) (`self.Distance between`))) 0.0 (`KismetMathLibrary.RandomFloatInRange` -1.0 -3.0)) (`KismetMathLibrary.MakeRotator` 0.0 (`KismetMathLibrary.RandomFloatInRange` -1.0 2.0))))))