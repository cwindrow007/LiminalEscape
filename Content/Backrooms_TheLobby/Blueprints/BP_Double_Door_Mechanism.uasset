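; BP_Double_Door_Mechanism is a double door prop for the Backrooms lobby level, posed through exposed values rather than animated at runtime.
; The construction script rolls each push-bar handle by its push amount and yaws each door by its open amount, negating the left door's yaw so the pair mirrors.
; The event graph holds no logic, so the doors have no scripted interaction or movement during play.
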(event `self.ReceiveTick`
  (params (DeltaSeconds :type "Float (single-precision)")))

(fn `UserConstructionScript`
  (`SceneComponent.K2_AddRelativeRotation` (`self.Left_Handle`) (`KismetMathLibrary.MakeRotator` (`self.Push_Left_Bar`)) false false)
  (`SceneComponent.K2_AddRelativeRotation` (`self.Left_Door`) (`KismetMathLibrary.MakeRotator` 0.0 0.0 (* -1 (`self.Open_Left_Door`))) false false)
  (`SceneComponent.K2_AddRelativeRotation` (`self.Right_Handle`) (`KismetMathLibrary.MakeRotator` (`self.Push_Right_Bar`)) false false)
  (`SceneComponent.K2_AddRelativeRotation` (`self.Right_Door`) (`KismetMathLibrary.MakeRotator` 0.0 0.0 (`self.Open_Right_Door`)) false false))