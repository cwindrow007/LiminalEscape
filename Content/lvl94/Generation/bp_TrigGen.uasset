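; Procedural terrain actor that builds a randomly bumpy grid mesh with collision when play begins.
; CreateVerts lays out an Xsize by Ysize grid with a random Z per vertex and scaled UVs.
; CreateTri stitches each cell into two triangles using a running vertex index that skips at row ends.
; Both arrays feed a ProceduralMesh section, created without supplied normals, which then receives the Material.
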(event `self.ReceiveBeginPlay`
  (`self.Create Verts`)
  (`self.Create Tri`)
  (`ProceduralMeshComponent.CreateMeshSection_LinearColor` :`self` (`self.ProceduralMesh`) :`Vertices` (`self.Vertices`) :`Triangles` (`self.Triangles`) :`UV0` (`self.UV0`) :`bCreateCollision` true)
  (`PrimitiveComponent.SetMaterial` (`self.ProceduralMesh`) 0 (`self.Material`)))

(fn `Create Tri`
  (locals (Vertex :type Integer))
  (for _ (range (`self.Xsize`))
    (for _ (range (`self.Ysize`))
      (`KismetArrayLibrary.Array_Add` (`self.Triangles`) (`local.Vertex`))
      (`KismetArrayLibrary.Array_Add` (`self.Triangles`) (+ (`local.Vertex`) 1))
      (`KismetArrayLibrary.Array_Add` (`self.Triangles`) (+ (`self.Ysize`) (`local.Vertex`) 1))
      (`KismetArrayLibrary.Array_Add` (`self.Triangles`) (+ (`local.Vertex`) 1))
      (`KismetArrayLibrary.Array_Add` (`self.Triangles`) (+ (`self.Ysize`) (`local.Vertex`) 2))
      (`KismetArrayLibrary.Array_Add` (`self.Triangles`) (+ (`self.Ysize`) (`local.Vertex`) 1))
      (`/Engine/EditorBlueprintResources/StandardMacros.IncrementInt` (`local.Vertex`)))
    (`/Engine/EditorBlueprintResources/StandardMacros.IncrementInt` (`local.Vertex`))))

(fn `Create Verts`
  (locals (X :type Integer) (Y :type Integer))
  (for _index (range (+ (`self.Xsize`) 1))
    (set `local.X` _index)
    (for _index_2 (range (+ (`self.Ysize`) 1))
      (set `local.Y` _index_2)
      (`KismetArrayLibrary.Array_Add` (`self.Vertices`) (`KismetMathLibrary.MakeVector` (* (`local.X`) (`self.Scale`)) (* (`local.Y`) (`self.Scale`)) (`KismetMathLibrary.RandomFloatInRange` (`self.Zmin`) (`self.Zmax`))))
      (`KismetArrayLibrary.Array_Add` (`self.UV0`) (`KismetMathLibrary.MakeVector2D` (* (`local.X`) (`self.UVScale`)) (* (`local.Y`) (`self.UVScale`)))))))

(fn `UserConstructionScript`)