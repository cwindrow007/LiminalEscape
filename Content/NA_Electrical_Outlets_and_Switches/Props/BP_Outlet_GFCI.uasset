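; BP_Outlet_GFCI is a configurable GFCI electrical outlet prop with customizable faceplate, outlet and screw finishes.
; The construction script creates a dynamic material instance for each of the three material slots on the SMFaceplateOutletGFCI mesh.
; Each instance takes its Color, Metallic and Roughness from that part's variables.
; The event graph holds only disabled placeholder events, so there is no runtime logic.
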(fn `UserConstructionScript`
  (bind _sm_faceplate_outlet_gfci (`self.SM_Faceplate_Outlet_GFCI`))
  (bind _returnvalue (`PrimitiveComponent.CreateDynamicMaterialInstance` _sm_faceplate_outlet_gfci 0 null "None"))
  (`MaterialInstanceDynamic.SetVectorParameterValue` _returnvalue "Color" (`self.FaceplateColor`))
  (`MaterialInstanceDynamic.SetScalarParameterValue` _returnvalue "Metallic" (`self.FaceplateMetallic`))
  (`MaterialInstanceDynamic.SetScalarParameterValue` _returnvalue "Roughness" (`self.FaceplateRoughness`))
  (bind _returnvalue_2 (`PrimitiveComponent.CreateDynamicMaterialInstance` _sm_faceplate_outlet_gfci 2 null "None"))
  (`MaterialInstanceDynamic.SetVectorParameterValue` _returnvalue_2 "Color" (`self.OutletColor`))
  (`MaterialInstanceDynamic.SetScalarParameterValue` _returnvalue_2 "Metallic" (`self.OutletMetallic`))
  (`MaterialInstanceDynamic.SetScalarParameterValue` _returnvalue_2 "Roughness" (`self.OutletRoughness`))
  (bind _returnvalue_3 (`PrimitiveComponent.CreateDynamicMaterialInstance` _sm_faceplate_outlet_gfci 1 null "None"))
  (`MaterialInstanceDynamic.SetVectorParameterValue` _returnvalue_3 "Color" (`self.Screw Color`))
  (`MaterialInstanceDynamic.SetScalarParameterValue` _returnvalue_3 "Metallic" (`self.Screw Metallic`))
  (`MaterialInstanceDynamic.SetScalarParameterValue` _returnvalue_3 "Roughness" (`self.Screw Roughness`)))