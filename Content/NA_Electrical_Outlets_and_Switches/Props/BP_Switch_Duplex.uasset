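; BP_Switch_Duplex is a duplex light switch prop with a faceplate mesh and two toggle switch child actors, with adjustable finishes.
; The construction script creates dynamic material instances for the faceplate's three slots, setting color, metallic and roughness for plate, screws and switch.
; It also casts each child actor to BP_Switch_Toggle and applies the switch finish to its skeletal mesh.
; The event graph contains no active logic.
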(fn `UserConstructionScript`
  (bind _sm_faceplate_switch_duplex (`self.SM_Faceplate_Switch_Duplex`))
  (bind _returnvalue (`PrimitiveComponent.CreateDynamicMaterialInstance` _sm_faceplate_switch_duplex 0 null "None"))
  (`MaterialInstanceDynamic.SetVectorParameterValue` _returnvalue "Color" (`self.FaceplateColor`))
  (`MaterialInstanceDynamic.SetScalarParameterValue` _returnvalue "Metallic" (`self.FaceplateMetallic`))
  (`MaterialInstanceDynamic.SetScalarParameterValue` _returnvalue "Roughness" (`self.FaceplateRoughness`))
  (bind _returnvalue_2 (`PrimitiveComponent.CreateDynamicMaterialInstance` _sm_faceplate_switch_duplex 1 null "None"))
  (`MaterialInstanceDynamic.SetVectorParameterValue` _returnvalue_2 "Color" (`self.ScrewColor`))
  (`MaterialInstanceDynamic.SetScalarParameterValue` _returnvalue_2 "Metallic" (`self.ScrewMetallic`))
  (`MaterialInstanceDynamic.SetScalarParameterValue` _returnvalue_2 "Roughness" (`self.ScrewRoughness`))
  (bind _returnvalue_3 (`PrimitiveComponent.CreateDynamicMaterialInstance` _sm_faceplate_switch_duplex 2 null "None"))
  (`MaterialInstanceDynamic.SetVectorParameterValue` _returnvalue_3 "Color" (`self.Switch Color`))
  (`MaterialInstanceDynamic.SetScalarParameterValue` _returnvalue_3 "Metallic" (`self.Switch Metallic`))
  (`MaterialInstanceDynamic.SetScalarParameterValue` _returnvalue_3 "Roughness" (`self.Switch Roughness`))
  (for _array_element (`|MakeArray` (`ChildActorComponent.ChildActor` (`self.BP_Switch_Toggle1`)) (`ChildActorComponent.ChildActor` (`self.BP_Switch_Toggle2`)))
    (bind _asbp_switch_toggle (cast `/Game/NA_Electrical_Outlets_and_Switches/Props/MovingParts/BP_Switch_Toggle` _array_element))
    (bind _returnvalue_4 (`PrimitiveComponent.CreateDynamicMaterialInstance` (`/Game/NA_Electrical_Outlets_and_Switches/Props/MovingParts/BP_Switch_Toggle.SK_Switch_Toggle` _asbp_switch_toggle) 0 null "None"))
    (`MaterialInstanceDynamic.SetVectorParameterValue` _returnvalue_4 "Color" (`self.Switch Color`))
    (`MaterialInstanceDynamic.SetScalarParameterValue` _returnvalue_4 "Metallic" (`self.Switch Metallic`))
    (`MaterialInstanceDynamic.SetScalarParameterValue` _returnvalue_4 "Roughness" (`self.Switch Roughness`))))