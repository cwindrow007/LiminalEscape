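; Slider light switch prop with a faceplate mesh and child actors for the slider and its button.
; The construction script creates dynamic material instances for the faceplate, screw and switch slots, driven by color, metallic and roughness variables.
; It casts to both child actors and applies the same switch finish to their meshes.
; The event graph has no active logic, so this Blueprint only handles appearance.
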(fn `UserConstructionScript`
  (bind _sm_faceplate_switch_slider (`self.SM_Faceplate_Switch_Slider`))
  (bind _switch_metallic (`self.Switch Metallic`))
  (bind _switch_color (`self.Switch Color`))
  (bind _switch_roughness (`self.Switch Roughness`))
  (bind _returnvalue (`PrimitiveComponent.CreateDynamicMaterialInstance` _sm_faceplate_switch_slider 0 null "None"))
  (`MaterialInstanceDynamic.SetVectorParameterValue` _returnvalue "Color" (`self.FaceplateColor`))
  (`MaterialInstanceDynamic.SetScalarParameterValue` _returnvalue "Metallic" (`self.FaceplateMetallic`))
  (`MaterialInstanceDynamic.SetScalarParameterValue` _returnvalue "Roughness" (`self.FaceplateRoughness`))
  (bind _returnvalue_2 (`PrimitiveComponent.CreateDynamicMaterialInstance` _sm_faceplate_switch_slider 1 null "None"))
  (`MaterialInstanceDynamic.SetVectorParameterValue` _returnvalue_2 "Color" (`self.Screw Color`))
  (`MaterialInstanceDynamic.SetScalarParameterValue` _returnvalue_2 "Metallic" (`self.Screw Metallic`))
  (`MaterialInstanceDynamic.SetScalarParameterValue` _returnvalue_2 "Roughness" (`self.Screw Roughness`))
  (bind _returnvalue_3 (`PrimitiveComponent.CreateDynamicMaterialInstance` _sm_faceplate_switch_slider 2 null "None"))
  (`MaterialInstanceDynamic.SetVectorParameterValue` _returnvalue_3 "Color" (`self.Switch Color`))
  (`MaterialInstanceDynamic.SetScalarParameterValue` _returnvalue_3 "Metallic" (`self.Switch Metallic`))
  (`MaterialInstanceDynamic.SetScalarParameterValue` _returnvalue_3 "Roughness" (`self.Switch Roughness`))
  (bind _asbp_slider (cast `/Game/NA_Electrical_Outlets_and_Switches/Props/MovingParts/BP_Slider` (`ChildActorComponent.ChildActor` (`self.BP_Slider`))))
  (bind _returnvalue_4 (`PrimitiveComponent.CreateDynamicMaterialInstance` (`/Game/NA_Electrical_Outlets_and_Switches/Props/MovingParts/BP_Slider.SwitchSlider_Slider` _asbp_slider) 0 null "None"))
  (`MaterialInstanceDynamic.SetVectorParameterValue` _returnvalue_4 "Color" _switch_color)
  (`MaterialInstanceDynamic.SetScalarParameterValue` _returnvalue_4 "Metallic" _switch_metallic)
  (`MaterialInstanceDynamic.SetScalarParameterValue` _returnvalue_4 "Roughness" _switch_roughness)
  (bind _asbp_slider_button (cast `/Game/NA_Electrical_Outlets_and_Switches/Props/MovingParts/BP_SliderButton` (`ChildActorComponent.ChildActor` (`self.BP_SliderButton`))))
  (bind _returnvalue_5 (`PrimitiveComponent.CreateDynamicMaterialInstance` (`/Game/NA_Electrical_Outlets_and_Switches/Props/MovingParts/BP_SliderButton.SwitchSlider_Button` _asbp_slider_button) 0 null "None"))
  (`MaterialInstanceDynamic.SetVectorParameterValue` _returnvalue_5 "Color" _switch_color)
  (`MaterialInstanceDynamic.SetScalarParameterValue` _returnvalue_5 "Metallic" _switch_metallic)
  (`MaterialInstanceDynamic.SetScalarParameterValue` _returnvalue_5 "Roughness" _switch_roughness))