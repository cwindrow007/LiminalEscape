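; BP_SMRADIO3 is an interactable radio prop that the player can silence once.
; Overlap events on its Sphere show and hide a Widget, with no filter on the overlapping actor.
; The Interact event runs through a DoOnce that hides the Widget, adds an audio component to the player character and instantly drops the radio's Audio volume to zero.
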(event `/Game/InteractInterface.Interact`
  (if true
    (`/Engine/EditorBlueprintResources/StandardMacros.DoOnce` false
      (:`Completed`
        (`SceneComponent.SetVisibility` (`self.Widget`) false false)
        (`AddComponent|NODE_AddAudioComponent-0` :`self` (`GameplayStatics.GetPlayerCharacter` 0))
        (`AudioComponent.AdjustVolume` (`self.Audio`) 0.0 0.0 "Linear")))))

(event `self.Sphere.OnComponentBeginOverlap`
  (params (OverlappedComponent :type "PrimitiveComponent Object Reference") (OtherActor :type "Actor Object Reference") (OtherComp :type "PrimitiveComponent Object Reference") (OtherBodyIndex :type Integer) (bFromSweep :type Boolean) (SweepResult :type "HitResult Structure (by ref)"))
  (`SceneComponent.SetVisibility` (`self.Widget`) true false))

(event `self.Sphere.OnComponentEndOverlap`
  (params (OverlappedComponent :type "PrimitiveComponent Object Reference") (OtherActor :type "Actor Object Reference") (OtherComp :type "PrimitiveComponent Object Reference") (OtherBodyIndex :type Integer))
  (`SceneComponent.SetVisibility` (`self.Widget`) false false))

(fn `UserConstructionScript`)