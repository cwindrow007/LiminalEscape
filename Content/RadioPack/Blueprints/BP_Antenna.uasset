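; BP_Antenna is a posable telescopic antenna prop from the RadioPack, configured in the editor with no active runtime logic.
; The construction script calls Setup, which pitches the base by ROTBase and rolls the antenna by ROTAntenna.
; A single Extend alpha lerps the relative Z of four sections between their retracted offsets and a shared ExtendDistance, telescoping them together.
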(fn `Setup`
  (bind _extenddistance (`self.ExtendDistance`))
  (`SceneComponent.K2_SetRelativeRotation` (`self.Antenna_Base`) (`KismetMathLibrary.MakeRotator` 0.0 (`self.ROTBase`)) false false)
  (`SceneComponent.K2_SetRelativeRotation` (`self.Antenna_A`) (`KismetMathLibrary.MakeRotator` (`self.ROTAntenna`)) false false)
  ;[1 1 1] If you wish to adjust each individual section replace "Extend" with "ExtendB1" "ExtendB2" etc
  (`SceneComponent.K2_SetRelativeLocation` (`self.Antenna_B1`) (`KismetMathLibrary.MakeVector` 0.0 0.0 (`KismetMathLibrary.Lerp` 2.4 _extenddistance (`self.Extend`))) false false)
  (`SceneComponent.K2_SetRelativeLocation` (`self.Antenna_B2`) (`KismetMathLibrary.MakeVector` 0.0 0.0 (`KismetMathLibrary.Lerp` 2.25 _extenddistance (`self.Extend`))) false false)
  (`SceneComponent.K2_SetRelativeLocation` (`self.Antenna_B3`) (`KismetMathLibrary.MakeVector` 0.0 0.0 (`KismetMathLibrary.Lerp` 2.25 _extenddistance (`self.Extend`))) false false)
  (`SceneComponent.K2_SetRelativeLocation` (`self.Antenna_B4`) (`KismetMathLibrary.MakeVector` 0.0 0.0 (`KismetMathLibrary.Lerp` 2.3 _extenddistance (`self.Extend`))) false false))

(fn `UserConstructionScript`
  (`self.Setup`))