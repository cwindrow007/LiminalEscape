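; BP_Radio is a configurable radio prop with a mesh, sound, optional child-actor antenna and play/stop events.
; The construction script sets up audio, passes rotation and extension settings to BP_Antenna, and runs Setup, which applies the mesh and a dynamic material instance with per-part colours.
; Setup can take its source material from the mesh automatically.
; UpdateVolume applies volume and rotates a supplied knob, switching axis for the Radio7 variant.
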(event `PlaySound`
  (bind _audio (`self.Audio`))
  ;[1 1 1] Play/Stop sound playing
  (if (not (`AudioComponent.IsPlaying` _audio))
    (`AudioComponent.Play` _audio 0.0)))

(event `StopSound`
  (bind _audio (`self.Audio`))
  ;[1 1 1] Play/Stop sound playing
  (if (`AudioComponent.IsPlaying` _audio)
    (`AudioComponent.Stop` _audio)))

(event `UpdateMaterial`
  ;[1 1 1] Get material from static mesh
  (set `self.Material` (`StaticMesh.GetMaterial` (`StaticMeshComponent.StaticMesh` (`self.Radio`)) 0))
  (`self.Setup`))

(fn `Setup`
  (bind _radio (`self.Radio`))
  (bind _radio_2 (`self.Radio`))
  (`StaticMeshComponent.SetStaticMesh` _radio_2 (`self.StaticMesh`))
  (`PrimitiveComponent.SetMaterial` _radio_2 1 (`self.MaterialDisplay`))
  (if (`self.bAutoUpdateMaterial`)
    (set `self.Material` (`StaticMesh.GetMaterial` (`StaticMeshComponent.StaticMesh` (`self.Radio`)) 0)))
  (bind _returnvalue (`PrimitiveComponent.CreateDynamicMaterialInstance` _radio 0 (`self.Material`) "None"))
  (set `self.DynamicMaterial` _returnvalue)
  (`PrimitiveComponent.SetMaterial` _radio 0 _returnvalue)
  (`MaterialInstanceDynamic.SetVectorParameterValue` _returnvalue "ColourCore" (`self.ColourCore`))
  (`MaterialInstanceDynamic.SetVectorParameterValue` _returnvalue "ColourShell" (`self.ColourShell`))
  (`MaterialInstanceDynamic.SetVectorParameterValue` _returnvalue "ColourPanel" (`self.ColourPanel`))
  (`MaterialInstanceDynamic.SetVectorParameterValue` _returnvalue "ColourButtons" (`self.ColourButtons`))
  (`MaterialInstanceDynamic.SetVectorParameterValue` _returnvalue "ColourSpeaker" (`self.ColourSpeaker`))
  (`MaterialInstanceDynamic.SetVectorParameterValue` _returnvalue "ColourText" (`self.ColourText`)))

(fn `UpdateVolume`
  (params (VolumeKnob :type "StaticMeshComponent Object Reference"))
  (`AudioComponent.SetVolumeMultiplier` (`self.Audio`) (`self.Volume`))
  (if (`KismetSystemLibrary.IsValid` VolumeKnob)
    (if (`self.bRadio7`)
      (`SceneComponent.K2_SetRelativeRotation` VolumeKnob (`KismetMathLibrary.MakeRotator` -90.0 0.0 (`KismetMathLibrary.Lerp` 120.0 0.0 (`self.Volume`))) false false)
      (else
        (`SceneComponent.K2_SetRelativeRotation` VolumeKnob (`KismetMathLibrary.MakeRotator` 0.0 (`KismetMathLibrary.Lerp` 120.0 0.0 (`self.Volume`)) 0.0) false false)))))

(fn `UserConstructionScript`
  (bind _audio (`self.Audio`))
  (bind _asbp_antenna (cast `/Game/RadioPack/Blueprints/BP_Antenna` (`ChildActorComponent.ChildActor` (`self.ChildActor`)) :!pure true))
  (`self.Setup`)
  (`AudioComponent.SetSound` _audio (`self.Sound`))
  (`AudioComponent.SetVolumeMultiplier` _audio (`self.Volume`))
  (`SceneComponent.SetVisibility` (`self.ChildActor`) (`self.bShowAntenna`) false)
  (set `/Game/RadioPack/Blueprints/BP_Antenna.ROTBase` (`self.ROTBase`) _asbp_antenna)
  (set `/Game/RadioPack/Blueprints/BP_Antenna.ROTAntenna` (`self.ROTAntenna`) _asbp_antenna)
  (set `/Game/RadioPack/Blueprints/BP_Antenna.Extend` (`self.Extend`) _asbp_antenna)
  (set `/Game/RadioPack/Blueprints/BP_Antenna.ExtendDistance` (`self.ExtendDistance`) _asbp_antenna)
  (`/Game/RadioPack/Blueprints/BP_Antenna.Setup` _asbp_antenna))