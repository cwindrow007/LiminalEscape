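; A fluorescent light fixture that flickers briefly and goes dark with a shattering effect the first time its ToggleLights event fires.
; The construction script sets the visibility of the tubes, cover, rect light and point light from the Ison flag.
; ToggleLights runs through a DoOnce, inverts that visibility twice with short delays, then hides those components, stops FluorideStare and plays LightbulbShattering.
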(event `self.ToggleLights`
  (`/Engine/EditorBlueprintResources/StandardMacros.DoOnce` false
    (:`Completed`
      (bind _output_get (set `self.Ison?` (not (`self.Ison?`))))
      (`SceneComponent.SetVisibility` (`self.Flourescent3`) _output_get false)
      (`SceneComponent.SetVisibility` (`self.Flourescent1`) _output_get false)
      (`SceneComponent.SetVisibility` (`self.RectLight`) _output_get false)
      (`SceneComponent.SetVisibility` (`self.Flourescent2`) _output_get false)
      (`SceneComponent.SetVisibility` (`self.Flourescent4`) _output_get false)
      (`SceneComponent.SetVisibility` (`self.Cover`) _output_get false)
      (`SceneComponent.SetVisibility` (`self.PointLight`) _output_get false)
      (`KismetSystemLibrary.Delay` 0.1)
      (bind _output_get_2 (set `self.Ison?` (not (`self.Ison`))))
      (`SceneComponent.SetVisibility` (`self.Flourescent3`) _output_get_2 false)
      (`SceneComponent.SetVisibility` (`self.Flourescent1`) _output_get_2 false)
      (`SceneComponent.SetVisibility` (`self.RectLight`) _output_get_2 false)
      (`SceneComponent.SetVisibility` (`self.Flourescent2`) _output_get_2 false)
      (`SceneComponent.SetVisibility` (`self.Flourescent4`) _output_get_2 false)
      (`SceneComponent.SetVisibility` (`self.Cover`) _output_get_2 false)
      (`SceneComponent.SetVisibility` (`self.PointLight`) _output_get_2 false)
      (`KismetSystemLibrary.Delay` 0.1)
      (set `self.Ison?` (not (`self.Ison`)))
      (`SceneComponent.SetVisibility` (`self.Flourescent4`) false false)
      (`SceneComponent.SetVisibility` (`self.Flourescent2`) false false)
      (`SceneComponent.SetVisibility` (`self.RectLight`) false false)
      (`SceneComponent.SetVisibility` (`self.Cover`) false false)
      (`SceneComponent.SetVisibility` (`self.Flourescent1`) false false)
      (`SceneComponent.SetVisibility` (`self.Flourescent3`) false false)
      (`SceneComponent.SetVisibility` (`self.PointLight`) false false)
      (`AudioComponent.Stop` (`self.FluorideStare`))
      (`AudioComponent.Play` (`self.LightbulbShattering`) 0.0))))

(fn `UserConstructionScript`
  (`SceneComponent.SetVisibility` (`self.Flourescent3`) (`self.Ison?`) false)
  (`SceneComponent.SetVisibility` (`self.Flourescent1`) (`self.Ison?`) false)
  (`SceneComponent.SetVisibility` (`self.Cover`) (`self.Ison?`) false)
  (`SceneComponent.SetVisibility` (`self.RectLight`) (`self.Ison?`) false)
  (`SceneComponent.SetVisibility` (`self.Flourescent2`) (`self.Ison?`) false)
  (`SceneComponent.SetVisibility` (`self.Flourescent4`) (`self.Ison?`) false)
  (`SceneComponent.SetVisibility` (`self.PointLight`) (`self.Ison?`) false))