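; Player character Blueprint with Enhanced Input movement, look, jump and sprint, plus a crosshair widget created on BeginPlay.
; Raw WASD key flags gate sprint to forward-only movement, resetting to walk speed for sideways or backward input.
; Tick drives a headbob by choosing idle, walk or sprint camera shakes from velocity.
; Died and DeathPit events ragdoll the Hazzy component, attach the camera to its pelvis, fade out and reload the level.
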(event `self.ReceiveBeginPlay`
  (bind _returnvalue (`GameplayStatics.GetPlayerCameraManager` 0))
  (`|ExecutionSequence`
    (:`then_0`
      (set `PlayerCameraManager.ViewPitchMin` -90.0 _returnvalue)
      (set `PlayerCameraManager.ViewPitchMax` 90.0 _returnvalue))
    (:`then_1`
      (`WidgetBlueprintLibrary.SetInputMode_GameOnly` (`GameplayStatics.GetPlayerController` 0))
      (bind _asgameplay_pc (cast `/Game/Blueprints/Gameplay_PC` (`self.GetController`)))
      (`/Engine/EditorBlueprintResources/StandardMacros.IsValid` _asgameplay_pc
        (:`Is Valid`
          (`EnhancedInputSubsystemInterface.AddMappingContext` (pcsubsystem `EnhancedInputLocalPlayerSubsystem` _asgameplay_pc) "/Game/Inputs/IMC_BaseInputs.IMC_BaseInputs" 0 (struct)))))
    (:`then_2`
      (bind _returnvalue_2 (`|GenericCreateObject` "/Game/BP_Crosshair.BP_Crosshair_C"))
      (`UserWidget.AddToViewport` _returnvalue_2 0))))

(event `EnhancedInput|/Game/Inputs/IA_Jump`
  (params (ActionValue :type Boolean) (ElapsedSeconds :type "Float (double-precision)") (TriggeredSeconds :type "Float (double-precision)") (InputAction :type "InputAction Object Reference" :default "/Game/Inputs/IA_Jump.IA_Jump"))
  ;[1 1 1] Jumpy Jump Jump
  (:`Triggered`
    (`self.Jump`)
    (set `CharacterMovementComponent.JumpZVelocity` 750.0 (`self.CharacterMovement`)))
  (:`Completed`
    (`self.StopJumping`)))

(event `Key|A`
  (params (Key :type "Key Structure"))
  ;[1 0 0] Sprinting
  (:`Pressed`
    (set `self.LeftPressed?` true))
  (:`Released`
    (set `self.LeftPressed?` false)))

(event `Key|D`
  (params (Key :type "Key Structure"))
  ;[1 0 0] Sprinting
  (:`Pressed`
    (set `self.RightPressed?` true))
  (:`Released`
    (set `self.RightPressed?` false)))

(event `Key|W`
  (params (Key :type "Key Structure"))
  ;[1 0 0] Sprinting
  (:`Pressed`
    (set `self.Forward Pressed?` true))
  (:`Released`
    (set `self.Forward Pressed?` false)))

(event `Key|S`
  (params (Key :type "Key Structure"))
  ;[1 0 0] Sprinting
  (:`Pressed`
    (set `self.BackwardPressed?` true))
  (:`Released`
    (set `self.BackwardPressed?` false)))

(event `EnhancedInput|/Game/Inputs/IA_Sprint`
  (params (ActionValue :type "Vector2D Structure") (ElapsedSeconds :type "Float (double-precision)") (TriggeredSeconds :type "Float (double-precision)") (InputAction :type "InputAction Object Reference" :default "/Game/Inputs/IA_Sprint.IA_Sprint"))
  (bind _charactermovement (`self.CharacterMovement`))
  ;[1 0 0] Sprinting
  (:`Triggered`
    (if (and (`self.Forward Pressed?`) (not (`self.BackwardPressed?`)))
      (set `CharacterMovementComponent.MaxWalkSpeed` (`self.SprintSpeed`) _charactermovement)
      (else
        (set `CharacterMovementComponent.MaxWalkSpeed` (`self.WalkSpeed`) _charactermovement :!label _label))))
  (:`Completed`
    (if true :!label _label_2
      (goto _label))))

(event `EnhancedInput|/Game/Inputs/IA_Sprint`
  (params (ActionValue :type "Vector2D Structure") (ElapsedSeconds :type "Float (double-precision)") (TriggeredSeconds :type "Float (double-precision)") (InputAction :type "InputAction Object Reference" :default "/Game/Inputs/IA_Sprint.IA_Sprint"))
  ;[1 0 0] Sprinting
  (:`Triggered`
    (if (`self.LeftPressed?`)
      (goto _label)))
  (:`Completed`
    (goto _label_2)))

(event `EnhancedInput|/Game/Inputs/IA_Look`
  (params (ActionValue :type "Vector2D Structure") (ElapsedSeconds :type "Float (double-precision)") (TriggeredSeconds :type "Float (double-precision)") (InputAction :type "InputAction Object Reference" :default "/Game/Inputs/IA_Look.IA_Look"))
  ;[1 0 0.8252] Mouse Movement
  (:`Triggered`
    (`self.AddControllerYawInput` ActionValue_X)
    (`self.AddControllerPitchInput` ActionValue_Y)))

(event `EnhancedInput|/Game/Inputs/IA_Sprint`
  (params (ActionValue :type "Vector2D Structure") (ElapsedSeconds :type "Float (double-precision)") (TriggeredSeconds :type "Float (double-precision)") (InputAction :type "InputAction Object Reference" :default "/Game/Inputs/IA_Sprint.IA_Sprint"))
  ;[1 0 0] Sprinting
  (:`Triggered`
    (if (`self.RightPressed?`)
      (goto _label)))
  (:`Completed`
    (goto _label_2)))

(event `EnhancedInput|/Game/Inputs/IA_Sprint`
  (params (ActionValue :type "Vector2D Structure") (ElapsedSeconds :type "Float (double-precision)") (TriggeredSeconds :type "Float (double-precision)") (InputAction :type "InputAction Object Reference" :default "/Game/Inputs/IA_Sprint.IA_Sprint"))
  ;[1 0 0] Sprinting
  (:`Triggered`
    (if (`self.BackwardPressed?`)
      (goto _label)))
  (:`Completed`
    (goto _label_2)))

(event `Headbob`
  (bind _returnvalue (`GameplayStatics.GetPlayerController` 0))
  (bind _returnvalue_2 (`KismetMathLibrary.VSize` (`self.GetVelocity`)))
  ;[0.01765 0.1458 0.1342 1 73] Headbob
  (if (and (> _returnvalue_2 0.0) (`self.CanJump`))
    (if (< _returnvalue_2 1200.0)
      (`PlayerController.ClientStartCameraShake` :`self` _returnvalue :`Shake` "/Game/WalkCameraShake.WalkCameraShake_C")
      (else
        (`PlayerController.ClientStartCameraShake` :`self` _returnvalue :`Shake` "/Game/SprintingCameraShake.SprintingCameraShake_C")))
    (else
      (`PlayerController.ClientStartCameraShake` :`self` _returnvalue :`Shake` "/Game/IdleCameraShake.IdleCameraShake_C"))))

(event `EnhancedInput|/Game/Inputs/IA_Move`
  (params (ActionValue :type "Vector2D Structure") (ElapsedSeconds :type "Float (double-precision)") (TriggeredSeconds :type "Float (double-precision)") (InputAction :type "InputAction Object Reference" :default "/Game/Inputs/IA_Move.IA_Move"))
  (bind (_returnvalue_roll _returnvalue_pitch _returnvalue_yaw) (`KismetMathLibrary.BreakRotator` (`self.GetControlRotation`)))
  (bind (_returnvalue_roll_2 _returnvalue_pitch_2 _returnvalue_yaw_2) (`KismetMathLibrary.BreakRotator` (`self.GetControlRotation`)))
  ;[0.1637 1 0.2953] Movement
  (:`Triggered`
    (`self.AddMovementInput` (`KismetMathLibrary.GetRightVector` (`KismetMathLibrary.MakeRotator` _returnvalue_roll_2 0.0 _returnvalue_yaw_2)) ActionValue_X)
    (`self.AddMovementInput` (`KismetMathLibrary.GetForwardVector` (`KismetMathLibrary.MakeRotator` 0.0 0.0 _returnvalue_yaw)) ActionValue_Y)))

(event `self.ReceiveTick`
  (params (DeltaSeconds :type "Float (single-precision)"))
  ;[0.01765 0.1458 0.1342 1 73] Headbob
  (`self.Headbob`))

(event `Died`
  (`CharacterMovementComponent.DisableMovement` (`self.CharacterMovement`))
  ;[1 1 1] KillBoxRespawn
  (`self.DisableInput` (`GameplayStatics.GetPlayerController` 0))
  (`PrimitiveComponent.SetSimulatePhysics` (`self.Hazzy`) true)
  (`SceneComponent.K2_AttachToComponent` (`self.Camera`) (`self.Hazzy`) "pelvis" "KeepRelative" "KeepRelative" "KeepRelative" true)
  (`PlayerCameraManager.StartCameraFade` :`self` (`GameplayStatics.GetPlayerCameraManager` 0) :`ToAlpha` 1.7 :`Duration` (`self.RespawnDuration`))
  (`KismetSystemLibrary.Delay` (`self.RespawnDuration`))
  (bind _returnvalue (`GameplayStatics.GetCurrentLevelName` true))
  (`GameplayStatics.OpenLevel` (`KismetStringLibrary.Conv_StringToName` _returnvalue)))

(event `DeathPit`
  (`CharacterMovementComponent.DisableMovement` (`self.CharacterMovement`))
  ;[1 1 1] Death Pit Respawn
  (`self.DisableInput` (`GameplayStatics.GetPlayerController` 0))
  (`PrimitiveComponent.SetSimulatePhysics` (`self.Hazzy`) true)
  (`SceneComponent.K2_AttachToComponent` (`self.Camera`) (`self.Hazzy`) "pelvis" "KeepRelative" "KeepRelative" "KeepRelative" true)
  (`PlayerCameraManager.StartCameraFade` :`self` (`GameplayStatics.GetPlayerCameraManager` 0) :`ToAlpha` 1.0 :`Duration` 2.0)
  (`KismetSystemLibrary.Delay` 2.0)
  (bind _returnvalue (`GameplayStatics.GetCurrentLevelName` true))
  (`GameplayStatics.OpenLevel` (`KismetStringLibrary.Conv_StringToName` _returnvalue)))

(fn `UserConstructionScript`)