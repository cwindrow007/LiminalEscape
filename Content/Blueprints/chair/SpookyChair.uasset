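; Spooky chair Blueprint that snaps its Chair component to a new rotation when a Character enters one of its trigger boxes.
; Each of the four overlap boxes sets its own fixed relative rotation, and does so on every entry.
; Boxes 1–2 and 3–4 each share a DoOnce leading to a common add-and-play audio step, so each pair triggers the sound only once.
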(event `self.box1.OnComponentBeginOverlap`
  (params (OverlappedComponent :type "PrimitiveComponent Object Reference") (OtherActor :type "Actor Object Reference") (OtherComp :type "PrimitiveComponent Object Reference") (OtherBodyIndex :type Integer) (bFromSweep :type Boolean) (SweepResult :type "HitResult Structure (by ref)"))
  (cast `Character` OtherActor)
  (`SceneComponent.K2_SetRelativeRotation` (`self.Chair`) (struct :`Yaw` 35.0) false false)
  (`/Engine/EditorBlueprintResources/StandardMacros.DoOnce` false :!label _label
    (:`Completed`
      (bind _returnvalue (`AddComponent|NODE_AddAudioComponent-1` :!label _label_2))
      (`AudioComponent.Play` _returnvalue 0.0))))

(event `self.box2.OnComponentBeginOverlap`
  (params (OverlappedComponent :type "PrimitiveComponent Object Reference") (OtherActor :type "Actor Object Reference") (OtherComp :type "PrimitiveComponent Object Reference") (OtherBodyIndex :type Integer) (bFromSweep :type Boolean) (SweepResult :type "HitResult Structure (by ref)"))
  (cast `Character` OtherActor)
  (`SceneComponent.K2_SetRelativeRotation` (`self.Chair`) (struct :`Yaw` 40.0) false false)
  (goto _label))

(event `self.box3.OnComponentBeginOverlap`
  (params (OverlappedComponent :type "PrimitiveComponent Object Reference") (OtherActor :type "Actor Object Reference") (OtherComp :type "PrimitiveComponent Object Reference") (OtherBodyIndex :type Integer) (bFromSweep :type Boolean) (SweepResult :type "HitResult Structure (by ref)"))
  (cast `Character` OtherActor)
  (`SceneComponent.K2_SetRelativeRotation` (`self.Chair`) (struct :`Yaw` 255.0) false false)
  (`/Engine/EditorBlueprintResources/StandardMacros.DoOnce` false :!label _label_3
    (:`Completed`
      (goto _label_2))))

(event `self.box4.OnComponentBeginOverlap`
  (params (OverlappedComponent :type "PrimitiveComponent Object Reference") (OtherActor :type "Actor Object Reference") (OtherComp :type "PrimitiveComponent Object Reference") (OtherBodyIndex :type Integer) (bFromSweep :type Boolean) (SweepResult :type "HitResult Structure (by ref)"))
  (cast `Character` OtherActor)
  (`SceneComponent.K2_SetRelativeRotation` (`self.Chair`) (struct :`Yaw` 245.0) false false)
  (goto _label_3))

(fn `UserConstructionScript`)