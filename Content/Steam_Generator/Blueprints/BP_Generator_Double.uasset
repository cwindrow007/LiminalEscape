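; Steam generator actor whose core animation spins up or winds down when a BaseCharacter overlaps its trigger.
; The core loops frozen at zero play rate from BeginPlay, and each accepted overlap toggles the steam valve's open or close animation.
; Two opposing gated Delay loops then gradually step the play rate toward full speed or stop, while a third gate enforces a cooldown between toggles.
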(event `self.ReceiveBeginPlay`
  (bind _generator_d_core (`self.Generator_D_core`))
  ;[1 1 1] Animation start and freeze
  (`self.EnableInput` (`GameplayStatics.GetPlayerController` 0))
  (`SkeletalMeshComponent.PlayAnimation` _generator_d_core "/Game/Steam_Generator/Meshes/Generator_double/Anim_Generator_D_core.Anim_Generator_D_core" true)
  (`SkeletalMeshComponent.SetPlayRate` _generator_d_core 0.0))

(event `Key|Two`
  (params (Key :type "Key Structure"))
  ;[1 1 1] INPUT
)

(event `self.Trigger.OnComponentBeginOverlap`
  (params (OverlappedComponent :type "PrimitiveComponent Object Reference") (OtherActor :type "Actor Object Reference") (OtherComp :type "PrimitiveComponent Object Reference") (OtherBodyIndex :type Integer) (bFromSweep :type Boolean) (SweepResult :type "HitResult Structure (by ref)"))
  (bind _generator_d_anim_speed (`self.Generator_D_anim_speed`))
  (bind _generator_d_anim_speed_2 (`self.Generator_D_anim_speed`))
  (cast `/Game/Blueprints/BaseCharacter` OtherActor)
  ;[1 1 1] Choice of engine start or stop, delay between commands
  (`/Engine/EditorBlueprintResources/StandardMacros.Gate` false :!label _label
    (:`Exit`
      (`|ExecutionSequence`
        (:`then_0`
          (if (`self.Steam_valve_D_open`)
            ;[1 1 1] Engine stop
            (`|ExecutionSequence`
              (:`then_0`
                (goto _label_3 :!via `Open`))
              (:`then_1`
                (goto _label_5 :!via `Close`))
              (:`then_2`
                (`SkeletalMeshComponent.PlayAnimation` (`self.Steam_valve`) "/Game/Steam_Generator/Meshes/Steam_valve/Anim_Steam_valve_close.Anim_Steam_valve_close" false)
                (set `self.Steam_valve_D_open` false)
                (`KismetSystemLibrary.Delay` 1.0)
                (`SkeletalMeshComponent.SetPlayRate` (`self.Generator_D_core`) _generator_d_anim_speed :!label _label_2)
                (`/Engine/EditorBlueprintResources/StandardMacros.Gate` true :!label _label_3
                  (:`Exit`
                    (`KismetSystemLibrary.Delay` 0.1)
                    (bind _result (`/Engine/EditorBlueprintResources/StandardMacros.ManipulateFloatInternal` _generator_d_anim_speed (- _generator_d_anim_speed 0.005))
                      (:`  `
                        (bind _output_get (set `self.Generator_D_anim_speed` _result))
                        (if (< _output_get 0.005)
                          (set `self.Generator_D_anim_speed` 0.0)
                          (`SkeletalMeshComponent.SetPlayRate` (`self.Generator_D_core`) _generator_d_anim_speed)
                          (else
                            (goto _label_2)))))))))
            (else
              ;[1 1 1] Engine acceleration
              (`|ExecutionSequence`
                (:`then_0`
                  (goto _label_5 :!via `Open`))
                (:`then_1`
                  (goto _label_3 :!via `Close`))
                (:`then_2`
                  (`SkeletalMeshComponent.PlayAnimation` (`self.Steam_valve`) "/Game/Steam_Generator/Meshes/Steam_valve/Anim_Steam_valve_open.Anim_Steam_valve_open" false)
                  (set `self.Steam_valve_D_open` true)
                  (`KismetSystemLibrary.Delay` 1.0)
                  (`SkeletalMeshComponent.SetPlayRate` (`self.Generator_D_core`) _generator_d_anim_speed_2 :!label _label_4)
                  (`/Engine/EditorBlueprintResources/StandardMacros.Gate` true :!label _label_5
                    (:`Exit`
                      (`KismetSystemLibrary.Delay` 0.1)
                      (bind _result_2 (`/Engine/EditorBlueprintResources/StandardMacros.ManipulateFloatInternal` _generator_d_anim_speed_2 (+ _generator_d_anim_speed_2 0.005))
                        (:`  `
                          (bind _output_get_2 (set `self.Generator_D_anim_speed` _result_2))
                          (if (< _output_get_2 1.0)
                            (goto _label_4)))))))))))
        (:`then_1`
          (goto _label :!via `Close`))
        (:`then_2`
          (`KismetSystemLibrary.Delay` 2.0)
          (goto _label :!via `Open`))))))

(fn `UserConstructionScript`)