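; Single steam generator Blueprint whose engine the player starts and stops with the 1 key.
; Each press toggles the steam valve open or closed with an animation, then after a short delay ramps the generator core's looping animation up or down.
; Two opposing Gate-and-Delay loops step the play rate gradually toward full speed or standstill, while a third Gate briefly blocks repeated key presses.
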(event `self.ReceiveBeginPlay`
  (bind _generator_s_core (`self.Generator_S_core`))
  ;[1 1 1] Animation start and freeze
  (`self.EnableInput` (`GameplayStatics.GetPlayerController` 0))
  (`SkeletalMeshComponent.PlayAnimation` _generator_s_core "/Game/Steam_Generator/Meshes/Generator_single/Anim_Generator_S_core.Anim_Generator_S_core" true)
  (`SkeletalMeshComponent.SetPlayRate` _generator_s_core 0.0))

(event `Key|One`
  (params (Key :type "Key Structure"))
  (bind _generator_s_anim_speed (`self.Generator_S_anim_speed`))
  (bind _generator_s_anim_speed_2 (`self.Generator_S_anim_speed`))
  ;[1 1 1] INPUT
  (:`Pressed`
    ;[1 1 1] Choice of engine start or stop, delay between commands
    (`/Engine/EditorBlueprintResources/StandardMacros.Gate` false :!label _label
      (:`Exit`
        (`|ExecutionSequence`
          (:`then_0`
            (if (`self.Steam_valve_S_open`)
              ;[1 1 1] Engine stop
              (`|ExecutionSequence`
                (:`then_0`
                  (goto _label_3 :!via `Open`))
                (:`then_1`
                  (goto _label_5 :!via `Close`))
                (:`then_2`
                  (`SkeletalMeshComponent.PlayAnimation` (`self.Steam_valve`) "/Game/Steam_Generator/Meshes/Steam_valve/Anim_Steam_valve_close.Anim_Steam_valve_close" false)
                  (set `self.Steam_valve_S_open` false)
                  (`KismetSystemLibrary.Delay` 1.0)
                  (`SkeletalMeshComponent.SetPlayRate` (`self.Generator_S_core`) _generator_s_anim_speed :!label _label_2)
                  (`/Engine/EditorBlueprintResources/StandardMacros.Gate` true :!label _label_3
                    (:`Exit`
                      (`KismetSystemLibrary.Delay` 0.1)
                      (bind _result (`/Engine/EditorBlueprintResources/StandardMacros.ManipulateFloatInternal` _generator_s_anim_speed (- _generator_s_anim_speed 0.005))
                        (:`  `
                          (bind _output_get (set `self.Generator_S_anim_speed` _result))
                          (if (< _output_get 0.005)
                            (set `self.Generator_S_anim_speed` 0.0)
                            (`SkeletalMeshComponent.SetPlayRate` (`self.Generator_S_core`) _generator_s_anim_speed)
                            (else
                              (goto _label_2)))))))))
              (else
                ;[1 1 1] Engine acceleration
                (`|ExecutionSequence`
                  (:`then_0`
                    (goto _label_5 :!via `Open`))
                  (:`then_1`
                    (goto _label_3 :!via `Close`))
                  (:`then_2`
                    (`SkeletalMeshComponent.PlayAnimation` (`self.Steam_valve`) "/Game/Steam_Generator/Meshes/Steam_valve/Anim_Steam_valve_open.Anim_Steam_valve_open" false)
                    (set `self.Steam_valve_S_open` true)
                    (`KismetSystemLibrary.Delay` 1.0)
                    (`SkeletalMeshComponent.SetPlayRate` (`self.Generator_S_core`) _generator_s_anim_speed_2 :!label _label_4)
                    (`/Engine/EditorBlueprintResources/StandardMacros.Gate` true :!label _label_5
                      (:`Exit`
                        (`KismetSystemLibrary.Delay` 0.1)
                        (bind _result_2 (`/Engine/EditorBlueprintResources/StandardMacros.ManipulateFloatInternal` _generator_s_anim_speed_2 (+ _generator_s_anim_speed_2 0.005))
                          (:`  `
                            (bind _output_get_2 (set `self.Generator_S_anim_speed` _result_2))
                            (if (< _output_get_2 1.0)
                              (goto _label_4)))))))))))
          (:`then_1`
            (goto _label :!via `Close`))
          (:`then_2`
            (`KismetSystemLibrary.Delay` 2.0)
            (goto _label :!via `Open`)))))))

(fn `UserConstructionScript`)