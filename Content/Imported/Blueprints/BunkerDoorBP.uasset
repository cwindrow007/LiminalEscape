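; BunkerDoorBP is an interactable bunker door that alternates between opening and closing through a FlipFlop, ignoring input while the valve timeline plays.
; Opening rolls the valve on one timeline, which after a Delay starts a second timeline that yaws the door.
; Closing reverses only the door timeline.
; Paired DoOnce gates reset each other to alternate handle and closing sounds, alongside a reactor door sound at fixed world coordinates.
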(event `/Game/InteractInterface.Interact`
  (if (not (`TimelineComponent.IsPlaying` (`self.Timeline`)))
    (`/Engine/EditorBlueprintResources/StandardMacros.FlipFlop`
      (:`A`
        (`|ExecutionSequence`
          (:`then_0`
            (`/Engine/EditorBlueprintResources/StandardMacros.DoOnce` false :!label _label
              (:`Completed`
                (`GameplayStatics.PlaySoundAtLocation` "/Game/Building/Blueprints/DoorHandle1.DoorHandle1" (0.0 0.0 0.0) (struct) 1.0 1.0 0.0 null null null null)
                (goto _label_3 :!via `Reset`))))
          (:`then_1`
            (`GameplayStatics.PlaySoundAtLocation` "/Game/Imported/Blueprints/ReactorDoor.ReactorDoor" (35735.367777 -49418.293058 379.493656) (struct) 1.0 1.0 0.0 null null null null)
            (bind (_direction _doorhandle) (`Timeline|Timeline`)
              (:`Update`
                (`SceneComponent.K2_SetRelativeRotation` (`self.Valve`) (`KismetMathLibrary.MakeRotator` (`KismetMathLibrary.Lerp` 0.0 -180.0 _doorhandle) 0.0 0.0) false false)
                (`KismetSystemLibrary.Delay` 0.5)
                (bind (_direction_2 _doormove) (`Timeline|Timeline_0` :!label _label_2)
                  (:`Update`
                    (`SceneComponent.K2_SetRelativeRotation` (`self.BunkerDoorNoValve`) (`KismetMathLibrary.MakeRotator` 0.0 0.0 (* _doormove 103.0)) false false))))))))
      (:`B`
        (`|ExecutionSequence`
          (:`then_0`
            (if (not (`TimelineComponent.IsPlaying` (`self.Timeline`)))
              (goto _label_2 :!via `Reverse`)))
          (:`then_1`
            (if (not (`TimelineComponent.IsReversing` (`self.Timeline`)))
              (`/Engine/EditorBlueprintResources/StandardMacros.DoOnce` false :!label _label_3
                (:`Completed`
                  (`GameplayStatics.PlaySoundAtLocation` "/Game/Building/Audio/Door_Closing.Door_Closing" (0.0 0.0 0.0) (struct) 1.0 1.0 0.0 null null null null)
                  (goto _label :!via `Reset`))))))))))

(fn `UserConstructionScript`)