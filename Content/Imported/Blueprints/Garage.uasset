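; Garage door actor that the player opens with the Interact event, raising a rolling gate mesh.
; A box overlap enables input on entry and disables it on exit, limiting interaction to that area.
; Interact passes a DoOnce, plays an opening sound at a hard-coded world location, and runs a Timeline that lerps the gate's relative location upward, with no closing logic.
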(event `/Game/InteractInterface.Interact`
  (`/Engine/EditorBlueprintResources/StandardMacros.DoOnce` false
    (:`Completed`
      (`GameplayStatics.PlaySoundAtLocation` "/Game/Imported/Blueprints/GarageOpening.GarageOpening" (30471.573274 -50740.797366 96.292294) (struct) 1.0 1.0 0.0 null null null null)
      (bind (_direction _newtrack_0) (`Timeline|Timeline`)
        (:`Update`
          (`SceneComponent.K2_SetRelativeLocation` (`self.Door_001_rolling-gate-g7c3d87256_1920_1`) (`KismetMathLibrary.VLerp` (0.0 0.0 0.0) (0.0 0.0 120.0) _newtrack_0) false false))))))

(event `self.Box.OnComponentBeginOverlap`
  (params (OverlappedComponent :type "PrimitiveComponent Object Reference") (OtherActor :type "Actor Object Reference") (OtherComp :type "PrimitiveComponent Object Reference") (OtherBodyIndex :type Integer) (bFromSweep :type Boolean) (SweepResult :type "HitResult Structure (by ref)"))
  (`self.EnableInput` (`GameplayStatics.GetPlayerController` 0) null))

(event `self.Box.OnComponentEndOverlap`
  (params (OverlappedComponent :type "PrimitiveComponent Object Reference") (OtherActor :type "Actor Object Reference") (OtherComp :type "PrimitiveComponent Object Reference") (OtherBodyIndex :type Integer))
  (`self.DisableInput` (`GameplayStatics.GetPlayerController` 0) null))

(fn `UserConstructionScript`)