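; DocumentPickupBP is a readable paper document in Level0 that the player opens and closes by interacting.
; Interact toggles on IsReading, playing a paper sound and either adding a widget of the configurable Class to the viewport or removing it.
; A BaseCharacter leaving InteractBox also removes the widget and resets the flag, without sound.
; The Pickup function is empty, with its note-flagging logic left disconnected.
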(event `self.ReceiveBeginPlay`
  (set `self.IsReading?` false))

(event `/Game/InteractInterface.Interact`
  (cast `/Game/Blueprints/BaseCharacter` (`GameplayStatics.GetPlayerCharacter` 0))
  (if (`self.IsReading?`)
    (`GameplayStatics.PlaySoundAtLocation` "/Game/Level0/Documents/PaperPickupCUE.PaperPickupCUE" (`SceneComponent.K2_GetComponentLocation` (`self.Paper`)) (struct) 1.0 1.0 0.0 null null null null)
    (`Widget.RemoveFromParent` (stale _returnvalue) :!label _label)
    (set `self.IsReading?` false)
    (else
      (`GameplayStatics.PlaySoundAtLocation` "/Game/Level0/Documents/PaperPickupCUE.PaperPickupCUE" (`SceneComponent.K2_GetComponentLocation` (`self.Paper`)) (struct) 1.0 1.0 0.0 null null null null)
      (bind _returnvalue (`|CreateWidget` (`self.Class`)))
      (`UserWidget.AddToViewport` _returnvalue 0)
      (set `self.IsReading?` true))))

(event `self.InteractBox.OnComponentEndOverlap`
  (params (OverlappedComponent :type "PrimitiveComponent Object Reference") (OtherActor :type "Actor Object Reference") (OtherComp :type "PrimitiveComponent Object Reference") (OtherBodyIndex :type Integer))
  (cast `/Game/Blueprints/BaseCharacter` OtherActor)
  (goto _label))

(fn `Pickup`
  (returns (StaticMesh :type "StaticMesh Object Reference") (NewParam :type "Actor Object Reference")))

(fn `UserConstructionScript`)