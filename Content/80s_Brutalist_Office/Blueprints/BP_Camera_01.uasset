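; BP_Camera_01 is a wall-mounted camera prop for the 80s Brutalist Office set, posed entirely in its Construction Script.
; Pitch and yaw variables rotate the camera body and its holder.
; Two splines then snap to left and right sockets on the wall holder and camera body, and spline mesh components follow them as connecting pieces, likely cables.
; The Event Graph holds no runtime logic.
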(fn `UserConstructionScript`
  (bind _spline_left (`self.Spline Left`))
  (bind _spline_right (`self.Spline Right`))
  (bind (_location _tangent) (`SplineComponent.GetLocationAndTangentAtSplinePoint` _spline_left 0 "Local"))
  (bind (_location_2 _tangent_2) (`SplineComponent.GetLocationAndTangentAtSplinePoint` _spline_left 1 "Local"))
  (bind (_location_3 _tangent_3) (`SplineComponent.GetLocationAndTangentAtSplinePoint` _spline_right 1 "Local"))
  (bind (_location_4 _tangent_4) (`SplineComponent.GetLocationAndTangentAtSplinePoint` _spline_right 0 "Local"))
  (`|ExecutionSequence`
    (:`then_0`
      (`SceneComponent.K2_AddLocalRotation` (`self.SM_Camera_01_Main_01`) (`KismetMathLibrary.MakeRotator` 0.0 (`self.Y (Pitch)`)) false false)
      (`SceneComponent.K2_AddLocalRotation` (`self.SM_Camera_01_Holder_02`) (`KismetMathLibrary.MakeRotator` 0.0 0.0 (`self.Z (Yaw)`)) false false))
    (:`then_1`
      (`SplineComponent.SetLocationAtSplinePoint` (`self.Spline Left`) 0 (`SceneComponent.GetSocketLocation` (`self.SM_Camera_01_Holder_01`) "Wall Left") "World" true)
      (`SplineComponent.SetLocationAtSplinePoint` (`self.Spline Left`) 1 (`SceneComponent.GetSocketLocation` (`self.SM_Camera_01_Main_01`) "Camera Left") "World" true)
      (`SplineComponent.SetLocationAtSplinePoint` (`self.Spline Right`) 0 (`SceneComponent.GetSocketLocation` (`self.SM_Camera_01_Holder_01`) "Wall Right") "World" true)
      (`SplineComponent.SetLocationAtSplinePoint` (`self.Spline Right`) 1 (`SceneComponent.GetSocketLocation` (`self.SM_Camera_01_Main_01`) "Camera Right") "World" true))
    (:`then_2`
      (bind _returnvalue (`AddComponent|NODE_AddSplineMeshComponent-0`))
      (`SplineMeshComponent.SetStartAndEnd` _returnvalue _location _tangent _location_2 _tangent_2 true)
      (bind _returnvalue_2 (`AddComponent|NODE_AddSplineMeshComponent-1`))
      (`SplineMeshComponent.SetStartAndEnd` _returnvalue_2 _location_4 _tangent_4 _location_3 _tangent_3 true))))