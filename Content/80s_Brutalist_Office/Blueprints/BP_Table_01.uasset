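; BP_Table_01 is an office table prop that randomizes its desks and chair in the construction script from a Seed random stream.
; Desk picks one of three desk meshes separately for each of two desk components.
; Chair moves the chair by either a fixed offset with a limited random yaw, or a random planar offset with any yaw.
; The event graph holds only disabled placeholder events, so the prop has no gameplay logic.
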(fn `Chair`
  (if (`KismetMathLibrary.RandomBoolFromStream` (`self.Seed`))
    (`SceneComponent.K2_AddLocalTransform` (`self.SM_Chair_01`) (`KismetMathLibrary.MakeTransform` (-50.0 15.0 0.0) (`KismetMathLibrary.MakeRotator` 0.0 0.0 (`KismetMathLibrary.RandomFloatInRangeFromStream` (`self.Seed`) 25.0 65.0))) false false)
    (else
      (`SceneComponent.K2_AddLocalTransform` (`self.SM_Chair_01`) (`KismetMathLibrary.MakeTransform` (`KismetMathLibrary.MakeVector` (`KismetMathLibrary.RandomFloatInRangeFromStream` (`self.Seed`) 0.0 40.0) (`KismetMathLibrary.RandomFloatInRangeFromStream` (`self.Seed`) 0.0 -40.0)) (`KismetMathLibrary.MakeRotator` 0.0 0.0 (`KismetMathLibrary.RandomFloatInRangeFromStream` (`self.Seed`) 0.0 360.0))) false false))))

(fn `Desk`
  (bind _output (`|GetArrayItem` (`|MakeArray` "/Game/80s_Brutalist_Office/Models/Desk/SM_Desk_02.SM_Desk_02" "/Game/80s_Brutalist_Office/Models/Desk/SM_Desk_03.SM_Desk_03" "/Game/80s_Brutalist_Office/Models/Desk/SM_Desk_04.SM_Desk_04" :!type "StaticMesh Object Reference") (`KismetMathLibrary.RandomIntegerInRangeFromStream` (`self.Seed`) 0 2)))
  (`StaticMeshComponent.SetStaticMesh` (`self.SM_Desk_03`) _output)
  (`StaticMeshComponent.SetStaticMesh` (`self.SM_Desk_02`) _output))

(fn `UserConstructionScript`
  (`|ExecutionSequence`
    (:`then_0`
      (`self.Desk`))
    (:`then_1`
      (`self.Chair`))))