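; Procedurally dressed office desk prop that randomizes its layout from a Seed stream in the Construction Script, with no runtime logic.
; Sub-functions jitter the PC, binders and chair, pick desk meshes, vary the monitor's atlas and scatter tinted sticky notes.
; A phone and a BP_Desk_Lamp_01 child actor take alternate spots, with configurable lamp light and material colors.
; The cigarette/prop step is disconnected, so it does nothing.
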(event `self.ReceiveBeginPlay`)

(fn `Chair`
  (if (`KismetMathLibrary.RandomBoolFromStream` (`self.Seed`))
    (`SceneComponent.K2_AddLocalTransform` (`self.SM_Chair_01`) (`KismetMathLibrary.MakeTransform` (-50.0 15.0 0.0) (`KismetMathLibrary.MakeRotator` 0.0 0.0 (`KismetMathLibrary.RandomFloatInRangeFromStream` (`self.Seed`) 25.0 65.0))) false false)
    (else
      (`SceneComponent.K2_AddLocalTransform` (`self.SM_Chair_01`) (`KismetMathLibrary.MakeTransform` (`KismetMathLibrary.MakeVector` (`KismetMathLibrary.RandomFloatInRangeFromStream` (`self.Seed`) 0.0 40.0) (`KismetMathLibrary.RandomFloatInRangeFromStream` (`self.Seed`) 0.0 -40.0)) (`KismetMathLibrary.MakeRotator` 0.0 0.0 (`KismetMathLibrary.RandomFloatInRangeFromStream` (`self.Seed`) 0.0 360.0))) false false))))

(fn `Cigarette/Prop`
  (locals (`Pick Location` :type Integer)))

(fn `Desk`
  (bind _output (`|GetArrayItem` (`|MakeArray` "/Game/80s_Brutalist_Office/Models/Desk/SM_Desk_02.SM_Desk_02" "/Game/80s_Brutalist_Office/Models/Desk/SM_Desk_03.SM_Desk_03" "/Game/80s_Brutalist_Office/Models/Desk/SM_Desk_04.SM_Desk_04" :!type "StaticMesh Object Reference") (`KismetMathLibrary.RandomIntegerInRangeFromStream` (`self.Seed`) 0 2)))
  (`StaticMeshComponent.SetStaticMesh` (`self.SM_Desk_03`) _output)
  (`StaticMeshComponent.SetStaticMesh` (`self.SM_Desk_02`) _output))

(fn `Desk Binder`
  (`SceneComponent.K2_AddLocalOffset` (`self.Desk Binder Left`) (`KismetMathLibrary.MakeVector` (`KismetMathLibrary.RandomFloatInRangeFromStream` (`self.Seed`) -35.0 35.0)) false true)
  (`SceneComponent.K2_AddLocalOffset` (`self.Desk Binder Right`) (`KismetMathLibrary.MakeVector` (`KismetMathLibrary.RandomFloatInRangeFromStream` (`self.Seed`) -35.0 35.0)) false true)
  (`SceneComponent.K2_AddLocalRotation` (`self.Desk Binder Right`) (`KismetMathLibrary.MakeRotator` 0.0 0.0 (`KismetMathLibrary.RandomFloatInRangeFromStream` (`self.Seed`) -10.0 10.0)) false false)
  (`SceneComponent.K2_AddLocalRotation` (`self.Desk Binder Left`) (`KismetMathLibrary.MakeRotator` 0.0 0.0 (`KismetMathLibrary.RandomFloatInRangeFromStream` (`self.Seed`) -10.0 10.0)) false false))

(fn `PC`
  (bind _returnvalue (`KismetMathLibrary.RandomIntegerInRangeFromStream` (`self.Seed`) 0 2))
  (bind _returnvalue_2 (`KismetMathLibrary.RandomFloatInRangeFromStream` (`self.Seed`) -20.0 20.0))
  (`|ExecutionSequence`
    (:`then_0`
      (`SceneComponent.K2_AddRelativeRotation` (`self.monitor`) (`KismetMathLibrary.MakeRotator` 0.0 0.0 (`KismetMathLibrary.RandomFloatInRangeFromStream` (`self.Seed`) -15.0 15.0)) false false)
      (`SceneComponent.K2_AddRelativeRotation` (`self.case`) (`KismetMathLibrary.MakeRotator` 0.0 0.0 (`KismetMathLibrary.RandomFloatInRangeFromStream` (`self.Seed`) -15.0 15.0)) false false)
      (`SceneComponent.K2_AddRelativeRotation` (`self.keyboard`) (`KismetMathLibrary.MakeRotator` 0.0 0.0 (`KismetMathLibrary.RandomFloatInRangeFromStream` (`self.Seed`) -15.0 15.0)) false false))
    (:`then_1`
      (for _ (range (+ (`|GetArrayItem` (`|MakeArray` _returnvalue _returnvalue _returnvalue _returnvalue) (`KismetMathLibrary.RandomIntegerInRangeFromStream` (`self.Seed`) 0 5)) 1))
        (bind _returnvalue_3 (`AddComponent|NODE_AddStaticMeshComponent-4` :`RelativeTransform` (`SceneComponent.GetRelativeTransform` (`self.monitor`))))
        (`SceneComponent.K2_AddLocalTransform` _returnvalue_3 (`KismetMathLibrary.MakeTransform` (-17.2 0.0 26.5) (struct :`Yaw` 90.0 :`Roll` -10.0) (1.3 1.3 1.3)) false false)
        (`SceneComponent.K2_AddLocalTransform` _returnvalue_3 (`KismetMathLibrary.MakeTransform` (`KismetMathLibrary.MakeVector` (`|GetArrayItem` (`|MakeArray` _returnvalue_2 _returnvalue_2 _returnvalue_2 _returnvalue_2) (`KismetMathLibrary.RandomIntegerInRangeFromStream` (`self.Seed`) 0 3))) (struct) (1.3 1.3 1.3)) false false)
        (`StaticMeshComponent.SetStaticMesh` _returnvalue_3 (`|GetArrayItem` (`|MakeArray` "/Game/80s_Brutalist_Office/Models/Paper_01/SM_StickyNote_01.SM_StickyNote_01" "/Game/80s_Brutalist_Office/Models/Paper_01/SM_StickyNote_02.SM_StickyNote_02" "/Game/80s_Brutalist_Office/Models/Paper_01/SM_StickyNote_03.SM_StickyNote_03" "/Game/80s_Brutalist_Office/Models/Paper_01/SM_StickyNote_04.SM_StickyNote_04" "/Game/80s_Brutalist_Office/Models/Paper_01/SM_StickyNote_05.SM_StickyNote_05" "/Game/80s_Brutalist_Office/Models/Paper_01/SM_StickyNote_06.SM_StickyNote_06" null null :!type "StaticMesh Object Reference") (`KismetMathLibrary.RandomIntegerInRangeFromStream` (`self.Seed`) 0 7)))
        (`PrimitiveComponent.SetMaterialByName` _returnvalue_3 "MI_Papers_01" (`|GetArrayItem` (`|MakeArray` "/Game/80s_Brutalist_Office/Models/Paper_01/MI_Papers_01_Pink.MI_Papers_01_Pink" "/Game/80s_Brutalist_Office/Models/Paper_01/MI_Papers_01_Yellow.MI_Papers_01_Yellow" :!type "MaterialInterface Object Reference") (`KismetMathLibrary.RandomIntegerInRangeFromStream` (`self.Seed`) 0 1)))))
    (:`then_2`
      (`MeshComponent.SetScalarParameterValueOnMaterials` (`self.monitor`) "Atlas Selector" (`KismetMathLibrary.RandomFloatInRangeFromStream` (`self.Seed`) 0.0 1.0)))))

(fn `Phone/Lamp`
  (locals (`Pick Location` :type Integer))
  (bind _lamp__light_color (`self.Lamp  Light Color`))
  (bind _pick_location (`local.Pick Location`))
  (bind _returnvalue (`KismetMathLibrary.MakeRotator` 0.0 0.0 (`KismetMathLibrary.RandomFloatInRangeFromStream` (`self.Seed`) -30.0 -70.0)))
  (`|ExecutionSequence`
    (:`then_0`
      (set `local.Pick Location` (`KismetMathLibrary.RandomIntegerInRangeFromStream` (`self.Seed`) 0 1)))
    (:`then_1`
      (`AddComponent|NODE_AddStaticMeshComponent-5` :`RelativeTransform` (`KismetMathLibrary.MakeTransform` (`|GetArrayItem` (`|MakeArray` (90.0 -25.0 71.2) (20.0 -95.0 71.2) :!type "Vector Structure") _pick_location) _returnvalue)))
    (:`then_2`
      (bind _returnvalue_2 (`AddComponent|NODE_AddChildActorComponent-0` :`RelativeTransform` (`KismetMathLibrary.MakeTransform` (`|GetArrayItem` (`|MakeArray` (20.0 -95.0 71.2) (90.0 -25.0 71.2) :!type "Vector Structure") _pick_location) _returnvalue)))
      (`SceneComponent.K2_AddLocalRotation` _returnvalue_2 (struct :`Yaw` 180.0) false false)
      (bind _asbp_desk_lamp_01 (cast `/Game/80s_Brutalist_Office/Blueprints/BP_Desk_Lamp_01` (`ChildActorComponent.ChildActor` _returnvalue_2)))
      (`LightComponent.SetLightColor` (`/Game/80s_Brutalist_Office/Blueprints/BP_Desk_Lamp_01.RectLight` _asbp_desk_lamp_01) _lamp__light_color true)
      (`LightComponent.SetLightColor` (`/Game/80s_Brutalist_Office/Blueprints/BP_Desk_Lamp_01.PointLight` _asbp_desk_lamp_01) _lamp__light_color true)
      (bind _sm_desk_lamp_01 (`/Game/80s_Brutalist_Office/Blueprints/BP_Desk_Lamp_01.SM_Desk_Lamp_01` _asbp_desk_lamp_01))
      (`MeshComponent.SetVectorParameterValueOnMaterials` _sm_desk_lamp_01 "Emissive Color" (`KismetMathLibrary.Conv_LinearColorToVector` _lamp__light_color))
      (`MeshComponent.SetVectorParameterValueOnMaterials` _sm_desk_lamp_01 "SSS Color" (`KismetMathLibrary.Conv_LinearColorToVector` (`self.Lamp SSS Color`))))))

(fn `UserConstructionScript`
  (`|ExecutionSequence`
    (:`then_0`
      (`self.PC`))
    (:`then_1`
      (`self.Desk`))
    (:`then_2`
      (`self.Phone/Lamp`))
    (:`then_3`
      (`self.Desk Binder`))
    (:`then_4`
      (`self.Chair`))
    (:`then_5`
      (`self.Cigarette/Prop`))))