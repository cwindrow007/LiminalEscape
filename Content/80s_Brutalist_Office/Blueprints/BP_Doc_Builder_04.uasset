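; Procedural office set-dressing actor that builds a random document prop, such as a colored binder, often topped with a small desk item.
; The Construction Script uses a random stream to pick one of four base variants, tinting the binder material in two of them.
; Depending on the variant, it always or randomly adds a notepad, mug, tape or pencil with jittered position and yaw.
; The event graph has no runtime logic.
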(fn `UserConstructionScript`
  (bind _stream (`self.Stream`))
  (bind _stream_2 (`self.Stream`))
  (bind _stream_3 (`self.Stream`))
  (bind _stream_4 (`self.Stream`))
  (bind _returnvalue (`KismetMathLibrary.RandomFloatInRangeFromStream` _stream -5.0 5.0))
  (bind _returnvalue_2 (`KismetMathLibrary.RandomFloatInRangeFromStream` _stream_2 -5.0 5.0))
  (bind _returnvalue_3 (`KismetMathLibrary.RandomFloatInRangeFromStream` _stream_3 -5.0 5.0))
  (bind _returnvalue_4 (`KismetMathLibrary.RandomFloatInRangeFromStream` _stream_4 -5.0 5.0))
  (switch `int` (`KismetMathLibrary.RandomIntegerInRangeFromStream` (`self.Stream`) 0 3)
    (:`0`
      (bind _returnvalue_5 (`AddComponent|NODE_AddStaticMeshComponent-0`))
      (`PrimitiveComponent.SetMaterialByName` _returnvalue_5 "MI_Document_Binder_01" (`|GetArrayItem` (`|MakeArray` "/Game/80s_Brutalist_Office/Models/Document_Binder_01/MI_Document_Binder_01_Orange.MI_Document_Binder_01_Orange" "/Game/80s_Brutalist_Office/Models/Document_Binder_01/MI_Document_Binder_01_Black.MI_Document_Binder_01_Black" "/Game/80s_Brutalist_Office/Models/Document_Binder_01/MI_Document_Binder_01_Green.MI_Document_Binder_01_Green" "/Game/80s_Brutalist_Office/Models/Document_Binder_01/MI_Document_Binder_01_Orange.MI_Document_Binder_01_Orange" "/Game/80s_Brutalist_Office/Models/Document_Binder_01/MI_Document_Binder_01_Yellow.MI_Document_Binder_01_Yellow" :!type "MaterialInterface Object Reference") (`KismetMathLibrary.RandomIntegerInRangeFromStream` (`self.Stream`) 0 4)))
      (bind _returnvalue_6 (`AddComponent|NODE_AddStaticMeshComponent-7` :`RelativeTransform` (`KismetMathLibrary.MakeTransform` (`KismetMathLibrary.MakeVector` _returnvalue_4 _returnvalue_4 1.0) (`KismetMathLibrary.MakeRotator` 0.0 0.0 (`KismetMathLibrary.RandomFloatInRangeFromStream` _stream_4 0.0 360.0)))))
      (`StaticMeshComponent.SetStaticMesh` _returnvalue_6 (`|GetArrayItem` (`|MakeArray` "/Game/80s_Brutalist_Office/Models/Notepad_01/SM_Notepad_01.SM_Notepad_01" "/Game/80s_Brutalist_Office/Models/Mug/SM_Mug_01.SM_Mug_01" :!type "StaticMesh Object Reference") (`KismetMathLibrary.RandomIntegerFromStream` (`self.Stream`) 3))))
    (:`1`
      (bind _returnvalue_7 (`AddComponent|NODE_AddStaticMeshComponent-1`))
      (`PrimitiveComponent.SetMaterialByName` _returnvalue_7 "MI_Document_Binder_01" (`|GetArrayItem` (`|MakeArray` "/Game/80s_Brutalist_Office/Models/Document_Binder_01/MI_Document_Binder_01_Orange.MI_Document_Binder_01_Orange" "/Game/80s_Brutalist_Office/Models/Document_Binder_01/MI_Document_Binder_01_Black.MI_Document_Binder_01_Black" "/Game/80s_Brutalist_Office/Models/Document_Binder_01/MI_Document_Binder_01_Green.MI_Document_Binder_01_Green" "/Game/80s_Brutalist_Office/Models/Document_Binder_01/MI_Document_Binder_01_Orange.MI_Document_Binder_01_Orange" "/Game/80s_Brutalist_Office/Models/Document_Binder_01/MI_Document_Binder_01_Yellow.MI_Document_Binder_01_Yellow" :!type "MaterialInterface Object Reference") (`KismetMathLibrary.RandomIntegerInRangeFromStream` (`self.Stream`) 0 4)))
      (if (`KismetMathLibrary.RandomBoolFromStream` _stream_3)
        (bind _returnvalue_8 (`AddComponent|NODE_AddStaticMeshComponent-6` :`RelativeTransform` (`KismetMathLibrary.MakeTransform` (`KismetMathLibrary.MakeVector` _returnvalue_3 _returnvalue_3 1.0) (`KismetMathLibrary.MakeRotator` 0.0 0.0 (`KismetMathLibrary.RandomFloatInRangeFromStream` _stream_3 0.0 360.0)))))
        (`StaticMeshComponent.SetStaticMesh` _returnvalue_8 (`|GetArrayItem` (`|MakeArray` "/Game/80s_Brutalist_Office/Models/DeskTape_01/SM_DeskTape_01.SM_DeskTape_01" "/Game/80s_Brutalist_Office/Models/Pencil_01/SM_Pencil_01.SM_Pencil_01" "/Game/80s_Brutalist_Office/Models/Mug/SM_Mug_01.SM_Mug_01" :!type "StaticMesh Object Reference") (`KismetMathLibrary.RandomIntegerFromStream` (`self.Stream`) 3)))))
    (:`2`
      (`AddComponent|NODE_AddStaticMeshComponent-2`)
      (if (`KismetMathLibrary.RandomBoolFromStream` _stream)
        (bind _returnvalue_9 (`AddComponent|NODE_AddStaticMeshComponent-4` :`RelativeTransform` (`KismetMathLibrary.MakeTransform` (`KismetMathLibrary.MakeVector` _returnvalue _returnvalue 0.5) (`KismetMathLibrary.MakeRotator` 0.0 0.0 (`KismetMathLibrary.RandomFloatInRangeFromStream` _stream 0.0 360.0)))))
        (`StaticMeshComponent.SetStaticMesh` _returnvalue_9 (`|GetArrayItem` (`|MakeArray` "/Game/80s_Brutalist_Office/Models/Pencil_01/SM_Pencil_01.SM_Pencil_01" "/Game/80s_Brutalist_Office/Models/Mug/SM_Mug_01.SM_Mug_01" :!type "StaticMesh Object Reference") (`KismetMathLibrary.RandomIntegerFromStream` (`self.Stream`) 2)))))
    (:`3`
      (`AddComponent|NODE_AddStaticMeshComponent-3`)
      (bind _returnvalue_10 (`AddComponent|NODE_AddStaticMeshComponent-5` :`RelativeTransform` (`KismetMathLibrary.MakeTransform` (`KismetMathLibrary.MakeVector` _returnvalue_2 _returnvalue_2 1.0) (`KismetMathLibrary.MakeRotator` 0.0 0.0 (`KismetMathLibrary.RandomFloatInRangeFromStream` _stream_2 0.0 360.0)))))
      (`StaticMeshComponent.SetStaticMesh` _returnvalue_10 (`|GetArrayItem` (`|MakeArray` "/Game/80s_Brutalist_Office/Models/Pencil_01/SM_Pencil_01.SM_Pencil_01" "/Game/80s_Brutalist_Office/Models/Mug/SM_Mug_01.SM_Mug_01" :!type "StaticMesh Object Reference") (`KismetMathLibrary.RandomIntegerFromStream` (`self.Stream`) 2))))))