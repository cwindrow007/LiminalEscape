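; Office set-dressing prop that procedurally builds a random arrangement of document binders in its Construction Script.
; A seeded random stream picks one of three layouts: a centered row with a count-scaled extra mesh, an alternating stack sometimes given a desk prop, or a slightly twisted stack.
; The same Seed drives counts, mesh variants, rotations and per-slot material colors, so each seed gives a repeatable result with no runtime logic.
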(event `self.ReceiveBeginPlay`)

(fn `Doc_01`
  (locals (`Docs Count` :type Integer :default 0))
  (bind _docs_count (`local.Docs Count`))
  (set `local.Docs Count` (`KismetMathLibrary.RandomIntegerInRangeFromStream` (`self.Seed`) 1 5))
  (for _index (range 1 (+ _docs_count 1))
    (bind _returnvalue (`AddComponent|NODE_AddStaticMeshComponent-0` :`RelativeTransform` (`KismetMathLibrary.MakeTransform` (`KismetMathLibrary.MakeVector` 0.0 (* (`KismetMathLibrary.Conv_IntToDouble` (- _index 1)) 8.5)))))
    (`SceneComponent.K2_AddLocalOffset` _returnvalue (`KismetMathLibrary.MakeVector` 0.0 (/ (* (`KismetMathLibrary.Conv_IntToDouble` (- _docs_count 1)) -8.5) 2.0)) false false)
    (`SceneComponent.K2_AddLocalRotation` _returnvalue (`KismetMathLibrary.MakeRotator` 0.0 0.0 (`|GetArrayItem` (`|MakeArray` 0.0 180.0 :!type "Float (single-precision)") (`KismetMathLibrary.RandomIntegerInRangeFromStream` (`self.Seed`) 0 1))) false false)
    (`StaticMeshComponent.SetStaticMesh` _returnvalue (`|GetArrayItem` (`|MakeArray` "/Game/80s_Brutalist_Office/Models/Document_Binder_03/SM_Document_Binder_03.SM_Document_Binder_03" "/Game/80s_Brutalist_Office/Models/Document_Binder_03/SM_Document_Binder_03_A.SM_Document_Binder_03_A" :!type "StaticMesh Object Reference") (`KismetMathLibrary.RandomIntegerInRangeFromStream` (`self.Seed`) 0 1)))
    (`PrimitiveComponent.SetMaterialByName` _returnvalue "MI_Document_Binder_03" (`|GetArrayItem` (`|MakeArray` "/Game/80s_Brutalist_Office/Models/Document_Binder_03/MI_Document_Binder_03.MI_Document_Binder_03" "/Game/80s_Brutalist_Office/Models/Document_Binder_03/MI_Document_Binder_03_Black.MI_Document_Binder_03_Black" "/Game/80s_Brutalist_Office/Models/Document_Binder_03/MI_Document_Binder_03_Green.MI_Document_Binder_03_Green" "/Game/80s_Brutalist_Office/Models/Document_Binder_03/MI_Document_Binder_03_Orange.MI_Document_Binder_03_Orange" "/Game/80s_Brutalist_Office/Models/Document_Binder_03/MI_Document_Binder_03_Yellow.MI_Document_Binder_03_Yellow" :!type "MaterialInterface Object Reference") (`KismetMathLibrary.RandomIntegerInRangeFromStream` (`self.Seed`) 0 4)))
    (`SceneComponent.K2_AddLocalRotation` _returnvalue (`KismetMathLibrary.MakeRotator` 0.0 0.0 (`KismetMathLibrary.RandomFloatInRangeFromStream` (`self.Seed`) -3.0 3.0)) false false))
  (`AddComponent|NODE_AddStaticMeshComponent-5` :`RelativeTransform` (`KismetMathLibrary.MakeTransform` (0.0 0.0 0.0) (struct) (`KismetMathLibrary.MakeVector` (* (`KismetMathLibrary.Conv_IntToDouble` (`local.Docs Count`)) 0.9) 2.75 3.45))))

(fn `Doc_02`
  (locals (`Doc Count` :type Integer :default 0))
  (bind _seed (`self.Seed`))
  (bind _returnvalue (`KismetMathLibrary.RandomFloatInRangeFromStream` _seed -5.0 5.0))
  (bind _output_get (set `local.Doc Count` (`KismetMathLibrary.RandomIntegerFromStream` (`self.Seed`) 3)))
  (for _index (range (+ _output_get 1))
    (bind _returnvalue_2 (`AddComponent|NODE_AddStaticMeshComponent-2`))
    (`SceneComponent.K2_AddLocalTransform` _returnvalue_2 (`KismetMathLibrary.MakeTransform` (`KismetMathLibrary.MakeVector` 0.0 0.0 (* (`KismetMathLibrary.Conv_IntToDouble` _index) 13.0)) (`KismetMathLibrary.MakeRotator` 0.0 0.0 (* (`KismetMathLibrary.Conv_IntToDouble` (+ _index 0)) 180.0))) false false)
    (`PrimitiveComponent.SetMaterialByName` _returnvalue_2 "MI_Document_Binder_03" (`|GetArrayItem` (`|MakeArray` "/Game/80s_Brutalist_Office/Models/Document_Binder_03/MI_Document_Binder_03.MI_Document_Binder_03" "/Game/80s_Brutalist_Office/Models/Document_Binder_03/MI_Document_Binder_03_Black.MI_Document_Binder_03_Black" "/Game/80s_Brutalist_Office/Models/Document_Binder_03/MI_Document_Binder_03_Green.MI_Document_Binder_03_Green" "/Game/80s_Brutalist_Office/Models/Document_Binder_03/MI_Document_Binder_03_Orange.MI_Document_Binder_03_Orange" "/Game/80s_Brutalist_Office/Models/Document_Binder_03/MI_Document_Binder_03_Yellow.MI_Document_Binder_03_Yellow" :!type "MaterialInterface Object Reference") (`KismetMathLibrary.RandomIntegerInRangeFromStream` (`self.Seed`) 0 4))))
  (if (`KismetMathLibrary.RandomBoolFromStream` _seed)
    (bind _returnvalue_3 (`AddComponent|NODE_AddStaticMeshComponent-6` :`RelativeTransform` (`KismetMathLibrary.MakeTransform` (`KismetMathLibrary.MakeVector` _returnvalue _returnvalue (* (`KismetMathLibrary.Conv_IntToDouble` _index) 13.0)) (`KismetMathLibrary.MakeRotator` 0.0 0.0 (`KismetMathLibrary.RandomFloatInRangeFromStream` _seed 0.0 360.0)))))
    (`StaticMeshComponent.SetStaticMesh` _returnvalue_3 (`|GetArrayItem` (`|MakeArray` "/Game/80s_Brutalist_Office/Models/Notepad_01/SM_Notepad_01.SM_Notepad_01" "/Game/80s_Brutalist_Office/Models/Pencil_01/SM_Pencil_01.SM_Pencil_01" "/Game/80s_Brutalist_Office/Models/Mug/SM_Mug_01.SM_Mug_01" :!type "StaticMesh Object Reference") (`KismetMathLibrary.RandomIntegerFromStream` (`self.Seed`) 3)))))

(fn `Doc_03`
  (bind _output (`|GetArrayItem` (`|MakeArray` "/Game/80s_Brutalist_Office/Models/Document_Binder_01/MI_Document_Binder_01.MI_Document_Binder_01" "/Game/80s_Brutalist_Office/Models/Document_Binder_01/MI_Document_Binder_01_Black.MI_Document_Binder_01_Black" "/Game/80s_Brutalist_Office/Models/Document_Binder_01/MI_Document_Binder_01_Green.MI_Document_Binder_01_Green" "/Game/80s_Brutalist_Office/Models/Document_Binder_01/MI_Document_Binder_01_Orange.MI_Document_Binder_01_Orange" "/Game/80s_Brutalist_Office/Models/Document_Binder_01/MI_Document_Binder_01_Yellow.MI_Document_Binder_01_Yellow" :!type "MaterialInterface Object Reference") (`KismetMathLibrary.RandomIntegerInRangeFromStream` (`self.Seed`) 0 4)))
  (for _index (range (+ (`KismetMathLibrary.RandomIntegerInRangeFromStream` (`self.Seed`) 0 3) 1))
    (bind _returnvalue (`AddComponent|NODE_AddStaticMeshComponent-3` :`RelativeTransform` (`KismetMathLibrary.MakeTransform` (`KismetMathLibrary.MakeVector` 0.0 0.0 (* (`KismetMathLibrary.Conv_IntToDouble` _index) 9.0)) (`KismetMathLibrary.MakeRotator` 0.0 0.0 (`KismetMathLibrary.RandomFloatInRangeFromStream` (`self.Seed`) -5.0 5.0)))))
    (`PrimitiveComponent.SetMaterialByName` _returnvalue "MI_Document_Binder_01" _output)
    (`PrimitiveComponent.SetMaterialByName` _returnvalue "MI_Document_Binder_01_Black" _output)
    (`PrimitiveComponent.SetMaterialByName` _returnvalue "MI_Document_Binder_01_Green" _output)
    (`PrimitiveComponent.SetMaterialByName` _returnvalue "MI_Document_Binder_01_Yellow" _output)
    (`PrimitiveComponent.SetMaterialByName` _returnvalue "MI_Document_Binder_01_Orange" _output)))

(fn `UserConstructionScript`
  (switch `int` (`KismetMathLibrary.RandomIntegerInRangeFromStream` (`self.Seed`) 0 2)
    (:`0`
      (`self.Doc_01`))
    (:`1`
      (`self.Doc_02`))
    (:`2`
      (`self.Doc_03`))))