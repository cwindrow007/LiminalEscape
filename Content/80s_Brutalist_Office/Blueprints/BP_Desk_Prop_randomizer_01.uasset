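; Desk prop randomizer that builds a varied cluster of office clutter from static mesh components in its construction script.
; A Seed random stream drives stack counts, yaw jitter and small offsets, keeping each layout repeatable.
; It adds a base mesh, two stacks, sticky notes with random mesh and color, and three single props, two with random paper colors.
; Sticky note height derives from the first stack's loop index; the event graph is unused.
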(fn `UserConstructionScript`
  (locals (NewLocalVar :type "Actor Object Reference"))
  (bind _returnvalue (`KismetMathLibrary.RandomFloatInRangeFromStream` (`self.Seed`) -8.0 8.0))
  (bind _returnvalue_2 (`KismetMathLibrary.MakeRotator` 0.0 0.0 (`KismetMathLibrary.RandomFloatInRangeFromStream` (`self.Seed`) -10.0 10.0)))
  (bind _output (`|GetArrayItem` (`|MakeArray` "/Game/80s_Brutalist_Office/Models/Paper_01/MI_Papers_01_Pink.MI_Papers_01_Pink" "/Game/80s_Brutalist_Office/Models/Paper_01/MI_Papers_01_Yellow.MI_Papers_01_Yellow" "/Game/80s_Brutalist_Office/Models/Paper_01/MI_Papers_01_Blue.MI_Papers_01_Blue" :!type "MaterialInterface Object Reference") (`KismetMathLibrary.RandomIntegerInRangeFromStream` (`self.Seed`) 0 2)))
  (`|ExecutionSequence`
    (:`then_0`
      (`AddComponent|NODE_AddStaticMeshComponent-4`))
    (:`then_1`
      (for _index (range (+ (`KismetMathLibrary.RandomIntegerInRangeFromStream` (`self.Seed`) 0 2) 1))
        (bind _returnvalue_3 (+ (* (`KismetMathLibrary.Conv_IntToDouble` _index) 0.85) 1.0))
        (`AddComponent|NODE_AddStaticMeshComponent-5` :`RelativeTransform` (`KismetMathLibrary.MakeTransform` (`KismetMathLibrary.MakeVector` 0.0 2.5 _returnvalue_3) (`KismetMathLibrary.MakeRotator` 0.0 0.0 (`KismetMathLibrary.RandomFloatInRangeFromStream` (`self.Seed`) 170.0 190.0)))))
      (for _ (range (+ (`KismetMathLibrary.RandomIntegerInRangeFromStream` (`self.Seed`) 0 3) 1))
        (bind _returnvalue_4 (`AddComponent|NODE_AddStaticMeshComponent-6` :`RelativeTransform` (`KismetMathLibrary.MakeTransform` (`KismetMathLibrary.MakeVector` _returnvalue _returnvalue _returnvalue_3) (`KismetMathLibrary.MakeRotator` -90.0 0.0 _returnvalue))))
        (`StaticMeshComponent.SetStaticMesh` _returnvalue_4 (`|GetArrayItem` (`|MakeArray` "/Game/80s_Brutalist_Office/Models/Paper_01/SM_StickyNote_01.SM_StickyNote_01" "/Game/80s_Brutalist_Office/Models/Paper_01/SM_StickyNote_02.SM_StickyNote_02" "/Game/80s_Brutalist_Office/Models/Paper_01/SM_StickyNote_03.SM_StickyNote_03" "/Game/80s_Brutalist_Office/Models/Paper_01/SM_StickyNote_04.SM_StickyNote_04" :!type "StaticMesh Object Reference") (`KismetMathLibrary.RandomIntegerInRangeFromStream` (`self.Seed`) 0 3)))
        (`PrimitiveComponent.SetMaterialByName` _returnvalue_4 "MI_Papers_01" (`|GetArrayItem` (`|MakeArray` "/Game/80s_Brutalist_Office/Models/Paper_01/MI_Papers_01_Pink.MI_Papers_01_Pink" "/Game/80s_Brutalist_Office/Models/Paper_01/MI_Papers_01_Yellow.MI_Papers_01_Yellow" "/Game/80s_Brutalist_Office/Models/Paper_01/MI_Papers_01_Blue.MI_Papers_01_Blue" :!type "MaterialInterface Object Reference") (`KismetMathLibrary.RandomIntegerInRangeFromStream` (`self.Seed`) 0 2)))))
    (:`then_2`
      (for _index_2 (range (+ (`KismetMathLibrary.RandomIntegerInRangeFromStream` (`self.Seed`) 0 2) 1))
        (`AddComponent|NODE_AddStaticMeshComponent-7` :`RelativeTransform` (`KismetMathLibrary.MakeTransform` (`KismetMathLibrary.MakeVector` 20.0 -8.0 (* (`KismetMathLibrary.Conv_IntToDouble` _index_2) 1.0)) (`KismetMathLibrary.MakeRotator` 0.0 0.0 (`KismetMathLibrary.RandomFloatInRangeFromStream` (`self.Seed`) -8.0 8.0))))))
    (:`then_3`
      (bind _returnvalue_5 (`AddComponent|NODE_AddStaticMeshComponent-8` :`RelativeTransform` (`KismetMathLibrary.MakeTransform` (17.0 5.0 0.0) _returnvalue_2)))
      (bind _returnvalue_6 (`AddComponent|NODE_AddStaticMeshComponent-9` :`RelativeTransform` (`KismetMathLibrary.MakeTransform` (17.0 13.0 0.0) _returnvalue_2)))
      (`PrimitiveComponent.SetMaterialByName` _returnvalue_6 "MI_Papers_02" _output)
      (`PrimitiveComponent.SetMaterialByName` _returnvalue_5 "MI_Papers_02" _output))
    (:`then_4`
      (`AddComponent|NODE_AddStaticMeshComponent-10` :`RelativeTransform` (`KismetMathLibrary.MakeTransform` (25.0 11.0 0.0) (`KismetMathLibrary.MakeRotator` 0.0 0.0 (`KismetMathLibrary.RandomFloatInRangeFromStream` (`self.Seed`) -10.0 10.0)))))))