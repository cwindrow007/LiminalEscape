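; Procedural smoking-clutter prop that assembles a randomized ashtray, cigarette box and Zippo arrangement in its Construction Script.
; The Seed stream drives a random ashtray yaw and coin flips for a mesh attached to the ashtray, a short box stack topped by another mesh, and an open or closed lighter.
; NewFunction duplicates the Construction Script logic, and the event graph holds only disabled stub events.
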(fn `NewFunction`
  (locals (`Ashtray Parent` :type "StaticMeshComponent Object Reference"))
  (`|ExecutionSequence`
    (:`then_0`
      (bind _returnvalue (`AddComponent|NODE_AddStaticMeshComponent-6` :`RelativeTransform` (`KismetMathLibrary.MakeTransform` (0.0 0.0 0.0) (`KismetMathLibrary.MakeRotator` 0.0 0.0 (`KismetMathLibrary.RandomFloatInRangeFromStream` (`self.Seed`) 0.0 360.0)))))
      (set `local.Ashtray Parent` _returnvalue))
    (:`then_1`
      (if (`KismetMathLibrary.RandomBoolFromStream` (`self.Seed`))
        (bind _returnvalue_2 (`AddComponent|NODE_AddStaticMeshComponent-7` :`RelativeTransform` (`KismetMathLibrary.MakeTransform` (0.0 3.0 1.8) (struct :`Roll` -19.0))))
        (`SceneComponent.K2_AttachToComponent` _returnvalue_2 (`local.Ashtray Parent`) "None" "KeepRelative" "KeepRelative" "KeepRelative" true)))
    (:`then_2`
      (if (`KismetMathLibrary.RandomBoolFromStream` (`self.Seed`))
        (for _index (range (+ (`KismetMathLibrary.RandomIntegerInRangeFromStream` (`self.Seed`) 0 1) 1))
          (bind _returnvalue_3 (`KismetMathLibrary.Conv_IntToDouble` _index))
          (bind _returnvalue_4 (`AddComponent|NODE_AddStaticMeshComponent-8` :`RelativeTransform` (`KismetMathLibrary.MakeTransform` (`KismetMathLibrary.MakeVector` -12.0 0.0 (* _returnvalue_3 1.7)) (`KismetMathLibrary.MakeRotator` 0.0 0.0 (`KismetMathLibrary.RandomFloatInRangeFromStream` (`self.Seed`) -15.0 15.0)))))
          (`StaticMeshComponent.SetStaticMesh` _returnvalue_4 (`|GetArrayItem` (`|MakeArray` "/Game/80s_Brutalist_Office/Models/Cigarette_01/SM_Cigarette_01_Box_02.SM_Cigarette_01_Box_02" "/Game/80s_Brutalist_Office/Models/Cigarette_01/SM_Cigarette_01_Box_01.SM_Cigarette_01_Box_01" :!type "StaticMesh Object Reference") (`KismetMathLibrary.RandomIntegerInRangeFromStream` (`self.Seed`) 0 1))))
        (`AddComponent|NODE_AddStaticMeshComponent-10` :`RelativeTransform` (`KismetMathLibrary.MakeTransform` (`KismetMathLibrary.MakeVector` -12.0 0.0 (* _returnvalue_3 1.95)) (`KismetMathLibrary.MakeRotator` 0.0 0.0 (`KismetMathLibrary.RandomFloatInRangeFromStream` (`self.Seed`) -15.0 15.0))))))
    (:`then_3`
      (if (`KismetMathLibrary.RandomBoolFromStream` (`self.Seed`))
        (bind _returnvalue_5 (`AddComponent|NODE_AddStaticMeshComponent-9` :`RelativeTransform` (`KismetMathLibrary.MakeTransform` (0.0 12.0 0.0) (`KismetMathLibrary.MakeRotator` 0.0 0.0 (`KismetMathLibrary.RandomFloatInRangeFromStream` (`self.Seed`) -50.0 50.0)))))
        (`StaticMeshComponent.SetStaticMesh` _returnvalue_5 (`|GetArrayItem` (`|MakeArray` "/Game/80s_Brutalist_Office/Models/Zippo/SM_Zippo_Opened_01.SM_Zippo_Opened_01" "/Game/80s_Brutalist_Office/Models/Zippo/SM_Zippo_Closed_01.SM_Zippo_Closed_01" :!type "StaticMesh Object Reference") (`KismetMathLibrary.RandomIntegerInRangeFromStream` (`self.Seed`) 0 1)))))))

(fn `UserConstructionScript`
  (locals (`Ashtray Parent` :type "StaticMeshComponent Object Reference"))
  (`|ExecutionSequence`
    (:`then_0`
      (bind _returnvalue (`AddComponent|NODE_AddStaticMeshComponent-0` :`RelativeTransform` (`KismetMathLibrary.MakeTransform` (0.0 0.0 0.0) (`KismetMathLibrary.MakeRotator` 0.0 0.0 (`KismetMathLibrary.RandomFloatInRangeFromStream` (`self.Seed`) 0.0 360.0)))))
      (set `local.Ashtray Parent` _returnvalue))
    (:`then_1`
      (if (`KismetMathLibrary.RandomBoolFromStream` (`self.Seed`))
        (bind _returnvalue_2 (`AddComponent|NODE_AddStaticMeshComponent-1` :`RelativeTransform` (`KismetMathLibrary.MakeTransform` (0.0 3.0 1.8) (struct :`Roll` -19.0))))
        (`SceneComponent.K2_AttachToComponent` _returnvalue_2 (`local.Ashtray Parent`) "None" "KeepRelative" "KeepRelative" "KeepRelative" true)))
    (:`then_2`
      (if (`KismetMathLibrary.RandomBoolFromStream` (`self.Seed`))
        (for _index (range (+ (`KismetMathLibrary.RandomIntegerInRangeFromStream` (`self.Seed`) 0 1) 1))
          (bind _returnvalue_3 (`KismetMathLibrary.Conv_IntToDouble` _index))
          (bind _returnvalue_4 (`AddComponent|NODE_AddStaticMeshComponent-3` :`RelativeTransform` (`KismetMathLibrary.MakeTransform` (`KismetMathLibrary.MakeVector` -12.0 0.0 (* _returnvalue_3 1.7)) (`KismetMathLibrary.MakeRotator` 0.0 0.0 (`KismetMathLibrary.RandomFloatInRangeFromStream` (`self.Seed`) -15.0 15.0)))))
          (`StaticMeshComponent.SetStaticMesh` _returnvalue_4 (`|GetArrayItem` (`|MakeArray` "/Game/80s_Brutalist_Office/Models/Cigarette_01/SM_Cigarette_01_Box_02.SM_Cigarette_01_Box_02" "/Game/80s_Brutalist_Office/Models/Cigarette_01/SM_Cigarette_01_Box_01.SM_Cigarette_01_Box_01" :!type "StaticMesh Object Reference") (`KismetMathLibrary.RandomIntegerInRangeFromStream` (`self.Seed`) 0 1))))
        (`AddComponent|NODE_AddStaticMeshComponent-5` :`RelativeTransform` (`KismetMathLibrary.MakeTransform` (`KismetMathLibrary.MakeVector` -12.0 0.0 (* _returnvalue_3 1.95)) (`KismetMathLibrary.MakeRotator` 0.0 0.0 (`KismetMathLibrary.RandomFloatInRangeFromStream` (`self.Seed`) -15.0 15.0))))))
    (:`then_3`
      (if (`KismetMathLibrary.RandomBoolFromStream` (`self.Seed`))
        (bind _returnvalue_5 (`AddComponent|NODE_AddStaticMeshComponent-4` :`RelativeTransform` (`KismetMathLibrary.MakeTransform` (0.0 12.0 0.0) (`KismetMathLibrary.MakeRotator` 0.0 0.0 (`KismetMathLibrary.RandomFloatInRangeFromStream` (`self.Seed`) -50.0 50.0)))))
        (`StaticMeshComponent.SetStaticMesh` _returnvalue_5 (`|GetArrayItem` (`|MakeArray` "/Game/80s_Brutalist_Office/Models/Zippo/SM_Zippo_Opened_01.SM_Zippo_Opened_01" "/Game/80s_Brutalist_Office/Models/Zippo/SM_Zippo_Closed_01.SM_Zippo_Closed_01" :!type "StaticMesh Object Reference") (`KismetMathLibrary.RandomIntegerInRangeFromStream` (`self.Seed`) 0 1)))))))