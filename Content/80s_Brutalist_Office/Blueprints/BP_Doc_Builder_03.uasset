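; BP_Doc_Builder_03 is an office-dressing Blueprint that scatters a small, seeded random arrangement of paper documents.
; Its construction script calls Paper01, which spawns a row of randomly picked, flattened paper meshes with jittered spacing, offset and yaw.
; Each paper gets a randomly rotated companion component slightly lower and nearby, then shifts back along X to roughly center the row.
; The event graph is empty, and a random-bool gate is left unconnected.
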(fn `Paper 01`
  (locals (`Sticky Note 01` :type "StaticMesh Object Reference" :default null) (`Paper Count` :type Integer :default 0) (`Paper Distance` :type "Float (double-precision)"))
  (bind _returnvalue (`KismetMathLibrary.RandomFloatInRangeFromStream` (`self.Seed`) -5.0 5.0))
  (bind _output_get (set `local.Paper Count` (`KismetMathLibrary.RandomIntegerInRangeFromStream` (`self.Seed`) 1 4)))
  (for _index (range (+ _output_get 1))
    (bind _output_get_2 (set `local.Paper Distance` (`KismetMathLibrary.RandomFloatInRangeFromStream` (`self.Seed`) 4.0 10.0)))
    (bind _returnvalue_2 (`AddComponent|NODE_AddStaticMeshComponent-2` :`RelativeTransform` (`KismetMathLibrary.MakeTransform` (`KismetMathLibrary.MakeVector` (* (`KismetMathLibrary.Conv_IntToDouble` _index) _output_get_2) (`KismetMathLibrary.RandomFloatInRangeFromStream` (`self.Seed`) -8.0 8.0)) (`KismetMathLibrary.MakeRotator` 90.0 0.0 (`KismetMathLibrary.RandomFloatInRangeFromStream` (`self.Seed`) -20.0 20.0)))))
    (`StaticMeshComponent.SetStaticMesh` _returnvalue_2 (`|GetArrayItem` (`|MakeArray` "/Game/80s_Brutalist_Office/Models/Paper_01/SM_Paper_01.SM_Paper_01" "/Game/80s_Brutalist_Office/Models/Paper_01/SM_Paper_02.SM_Paper_02" "/Game/80s_Brutalist_Office/Models/Paper_01/SM_Paper_03.SM_Paper_03" "/Game/80s_Brutalist_Office/Models/Paper_01/SM_Paper_04.SM_Paper_04" "/Game/80s_Brutalist_Office/Models/Paper_01/SM_Paper_05.SM_Paper_05" "/Game/80s_Brutalist_Office/Models/Paper_01/SM_Paper_05.SM_Paper_05" :!type "StaticMesh Object Reference") (`KismetMathLibrary.RandomIntegerInRangeFromStream` (`self.Seed`) 0 5)))
    (`SceneComponent.K2_AddLocalTransform` _returnvalue_2 (`KismetMathLibrary.MakeTransform` (`KismetMathLibrary.MakeVector` 0.0 (* (`KismetMathLibrary.Conv_IntToDouble` (- _index 1)) 0.05)) (struct) (1.0 0.1 1.0)) false false)
    (bind _returnvalue_location (`KismetMathLibrary.BreakTransform` (`SceneComponent.GetRelativeTransform` _returnvalue_2)))
    (bind _returnvalue_3 (`AddComponent|NODE_AddStaticMeshComponent-6` :`RelativeTransform` (`KismetMathLibrary.MakeTransform` (`KismetMathLibrary.MakeVector` (+ (.x _returnvalue_location) _returnvalue) (+ (.y _returnvalue_location) _returnvalue) -0.15) (`KismetMathLibrary.MakeRotator` 0.0 0.0 (`KismetMathLibrary.RandomFloatInRangeFromStream` (`self.Seed`) 0.0 360.0)))))
    (`StaticMeshComponent.SetStaticMesh` _returnvalue_3 (`|GetArrayItem` (`|MakeArray` null null null null null null :!type "StaticMesh Object Reference") (`KismetMathLibrary.RandomIntegerInRangeFromStream` (`self.Seed`) 0 5)))
    (`SceneComponent.K2_AddLocalOffset` _returnvalue_2 (`KismetMathLibrary.MakeVector` (/ (* (`KismetMathLibrary.Conv_IntToDouble` (`local.Paper Count`)) (* (`local.Paper Distance`) -1.0)) 2.0)) false false)))

(fn `UserConstructionScript`
  (`self.Paper 01`))