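; Office set-dressing actor that procedurally builds a small cluster of papers and sticky notes laid out in the XZ plane.
; The construction script uses a seeded random stream to pick one of two layouts, with random counts, meshes and offsets.
; Paper01 makes an evenly spaced row with a note slot per sheet.
; Paper02 makes a tighter, depth-staggered overlap with one final note slot, which can stay empty; notes are pink or yellow.
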(fn `Paper_01`
  (locals (`Stick Note 01` :type "StaticMesh Object Reference" :default null) (`Paper Count` :type Integer :default 0))
  (bind _output_get (set `local.Paper Count` (`KismetMathLibrary.RandomIntegerInRangeFromStream` (`self.Seed`) 1 4)))
  (for _index (range 1 (+ _output_get 1))
    (bind _returnvalue (`AddComponent|NODE_AddStaticMeshComponent-0` :`RelativeTransform` (`KismetMathLibrary.MakeTransform` (`KismetMathLibrary.MakeVector` (+ (`KismetMathLibrary.RandomFloatInRangeFromStream` (`self.Seed`) -2.0 2.0) (* (`KismetMathLibrary.Conv_IntToDouble` _index) 24.0)) 0.0 (`KismetMathLibrary.RandomFloatInRangeFromStream` (`self.Seed`) -4.0 4.0)))))
    (`StaticMeshComponent.SetStaticMesh` _returnvalue (`|GetArrayItem` (`|MakeArray` "/Game/80s_Brutalist_Office/Models/Paper_01/SM_Paper_01.SM_Paper_01" "/Game/80s_Brutalist_Office/Models/Paper_01/SM_Paper_02.SM_Paper_02" "/Game/80s_Brutalist_Office/Models/Paper_01/SM_Paper_03.SM_Paper_03" "/Game/80s_Brutalist_Office/Models/Paper_01/SM_Paper_04.SM_Paper_04" "/Game/80s_Brutalist_Office/Models/Paper_01/SM_Paper_05.SM_Paper_05" "/Game/80s_Brutalist_Office/Models/Paper_01/SM_Paper_05.SM_Paper_05" :!type "StaticMesh Object Reference") (`KismetMathLibrary.RandomIntegerInRangeFromStream` (`self.Seed`) 0 5)))
    (bind _returnvalue_location (`KismetMathLibrary.BreakTransform` (`SceneComponent.GetRelativeTransform` _returnvalue)))
    (bind _returnvalue_2 (`AddComponent|NODE_AddStaticMeshComponent-3` :`RelativeTransform` (`KismetMathLibrary.MakeTransform` (`KismetMathLibrary.MakeVector` (+ (.x _returnvalue_location) (`KismetMathLibrary.RandomFloatInRangeFromStream` (`self.Seed`) -9.0 9.0)) (+ (.y _returnvalue_location) 0.2) (+ (.z _returnvalue_location) 10.0)) (struct) (1.3 1.3 1.3))))
    (`StaticMeshComponent.SetStaticMesh` _returnvalue_2 (`|GetArrayItem` (`|MakeArray` "/Game/80s_Brutalist_Office/Models/Paper_01/SM_StickyNote_01.SM_StickyNote_01" "/Game/80s_Brutalist_Office/Models/Paper_01/SM_StickyNote_02.SM_StickyNote_02" "/Game/80s_Brutalist_Office/Models/Paper_01/SM_StickyNote_03.SM_StickyNote_03" "/Game/80s_Brutalist_Office/Models/Paper_01/SM_StickyNote_04.SM_StickyNote_04" "/Game/80s_Brutalist_Office/Models/Paper_01/SM_StickyNote_05.SM_StickyNote_05" "/Game/80s_Brutalist_Office/Models/Paper_01/SM_StickyNote_06.SM_StickyNote_06" null null :!type "StaticMesh Object Reference") (`KismetMathLibrary.RandomIntegerInRangeFromStream` (`self.Seed`) 0 7)))
    (`SceneComponent.K2_AddLocalOffset` _returnvalue (`KismetMathLibrary.MakeVector` (/ (* (`KismetMathLibrary.Conv_IntToDouble` (+ (`local.Paper Count`) 1)) -24.0) 2.0)) false false)
    (`SceneComponent.K2_AddLocalOffset` _returnvalue_2 (`KismetMathLibrary.MakeVector` (/ (* (`KismetMathLibrary.Conv_IntToDouble` (+ (`local.Paper Count`) 1)) -24.0) 2.0)) false false)
    (`PrimitiveComponent.SetMaterialByName` _returnvalue_2 "MI_Papers_01" (`|GetArrayItem` (`|MakeArray` "/Game/80s_Brutalist_Office/Models/Paper_01/MI_Papers_01_Pink.MI_Papers_01_Pink" "/Game/80s_Brutalist_Office/Models/Paper_01/MI_Papers_01_Yellow.MI_Papers_01_Yellow" :!type "MaterialInterface Object Reference") (`KismetMathLibrary.RandomIntegerInRangeFromStream` (`self.Seed`) 0 1)))))

(fn `Paper_02`
  (locals (`Sticky Note 01` :type "StaticMesh Object Reference" :default "/Script/Engine.StaticMesh'/Game/80s_Brutalist_Office/Models/Paper_01/SM_StickyNote_01.SM_StickyNote_01'") (`Paper Count` :type Integer :default 0) (`Paper Distance` :type "Float (double-precision)"))
  (bind _output_get (set `local.Paper Count` (`KismetMathLibrary.RandomIntegerInRangeFromStream` (`self.Seed`) 1 6)))
  (for _index (range (+ _output_get 1))
    (bind _output_get_2 (set `local.Paper Distance` (`KismetMathLibrary.RandomFloatInRangeFromStream` (`self.Seed`) 4.0 16.0)))
    (bind _returnvalue (`AddComponent|NODE_AddStaticMeshComponent-2` :`RelativeTransform` (`KismetMathLibrary.MakeTransform` (`KismetMathLibrary.MakeVector` (* (`KismetMathLibrary.Conv_IntToDouble` _index) _output_get_2) 0.0 (`KismetMathLibrary.RandomFloatInRangeFromStream` (`self.Seed`) -4.0 4.0)))))
    (`StaticMeshComponent.SetStaticMesh` _returnvalue (`|GetArrayItem` (`|MakeArray` "/Game/80s_Brutalist_Office/Models/Paper_01/SM_Paper_01.SM_Paper_01" "/Game/80s_Brutalist_Office/Models/Paper_01/SM_Paper_02.SM_Paper_02" "/Game/80s_Brutalist_Office/Models/Paper_01/SM_Paper_03.SM_Paper_03" "/Game/80s_Brutalist_Office/Models/Paper_01/SM_Paper_04.SM_Paper_04" "/Game/80s_Brutalist_Office/Models/Paper_01/SM_Paper_05.SM_Paper_05" "/Game/80s_Brutalist_Office/Models/Paper_01/SM_Paper_05.SM_Paper_05" :!type "StaticMesh Object Reference") (`KismetMathLibrary.RandomIntegerInRangeFromStream` (`self.Seed`) 0 5)))
    (`SceneComponent.K2_AddLocalTransform` _returnvalue (`KismetMathLibrary.MakeTransform` (`KismetMathLibrary.MakeVector` 0.0 (* (`KismetMathLibrary.Conv_IntToDouble` (- _index 1)) 0.15))) false false)
    (`SceneComponent.K2_AddLocalOffset` (stale _returnvalue_2) (`KismetMathLibrary.MakeVector` (/ (* (`KismetMathLibrary.Conv_IntToDouble` (`local.Paper Count`)) (* (`local.Paper Distance`) -1.0)) 2.0)) false false)
    (`SceneComponent.K2_AddLocalOffset` _returnvalue (`KismetMathLibrary.MakeVector` (/ (* (`KismetMathLibrary.Conv_IntToDouble` (`local.Paper Count`)) (* (`local.Paper Distance`) -1.0)) 2.0)) false false))
  (bind _returnvalue_location (`KismetMathLibrary.BreakTransform` (`SceneComponent.GetRelativeTransform` _returnvalue)))
  (bind _returnvalue_2 (`AddComponent|NODE_AddStaticMeshComponent-5` :`RelativeTransform` (`KismetMathLibrary.MakeTransform` (`KismetMathLibrary.MakeVector` (+ (.x _returnvalue_location) (`KismetMathLibrary.RandomFloatInRangeFromStream` (`self.Seed`) -9.0 9.0)) (+ (.y _returnvalue_location) 0.2) (+ (.z _returnvalue_location) 10.0)) (struct) (1.3 1.3 1.3))))
  (`StaticMeshComponent.SetStaticMesh` _returnvalue_2 (`|GetArrayItem` (`|MakeArray` "/Game/80s_Brutalist_Office/Models/Paper_01/SM_StickyNote_01.SM_StickyNote_01" "/Game/80s_Brutalist_Office/Models/Paper_01/SM_StickyNote_02.SM_StickyNote_02" "/Game/80s_Brutalist_Office/Models/Paper_01/SM_StickyNote_03.SM_StickyNote_03" "/Game/80s_Brutalist_Office/Models/Paper_01/SM_StickyNote_04.SM_StickyNote_04" "/Game/80s_Brutalist_Office/Models/Paper_01/SM_StickyNote_05.SM_StickyNote_05" "/Game/80s_Brutalist_Office/Models/Paper_01/SM_StickyNote_06.SM_StickyNote_06" null null :!type "StaticMesh Object Reference") (`KismetMathLibrary.RandomIntegerInRangeFromStream` (`self.Seed`) 0 7)))
  (`PrimitiveComponent.SetMaterialByName` _returnvalue_2 "MI_Papers_01" (`|GetArrayItem` (`|MakeArray` "/Game/80s_Brutalist_Office/Models/Paper_01/MI_Papers_01_Pink.MI_Papers_01_Pink" "/Game/80s_Brutalist_Office/Models/Paper_01/MI_Papers_01_Yellow.MI_Papers_01_Yellow" :!type "MaterialInterface Object Reference") (`KismetMathLibrary.RandomIntegerInRangeFromStream` (`self.Seed`) 0 1))))

(fn `UserConstructionScript`
  (switch `int` (`KismetMathLibrary.RandomIntegerInRangeFromStream` (`self.Seed`) 0 1)
    (:`0`
      (`self.Paper_01`))
    (:`1`
      (`self.Paper_02`))))