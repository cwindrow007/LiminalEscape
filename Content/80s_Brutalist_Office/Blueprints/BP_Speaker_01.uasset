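; Wall speaker prop for the brutalist office set, with adjustable tilt and swivel and a cable that follows its pose.
; The construction script pitches the speaker body and yaws its holder from two variables, then snaps two spline points to cable sockets on the second holder mesh and the body.
; A spline mesh added at construction spans those points using their local positions and tangents.
; The event graph is empty.
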(fn `UserConstructionScript`
  (bind _spline (`self.Spline`))
  (bind (_location _tangent) (`SplineComponent.GetLocationAndTangentAtSplinePoint` _spline 1 "Local"))
  (bind (_location_2 _tangent_2) (`SplineComponent.GetLocationAndTangentAtSplinePoint` _spline 0 "Local"))
  (`|ExecutionSequence`
    (:`then_0`
      (`SceneComponent.K2_AddLocalRotation` (`self.SM_Speaker_01_Main_01`) (`KismetMathLibrary.MakeRotator` 0.0 (`self.Y (Pitch)`)) false false)
      (`SceneComponent.K2_AddLocalRotation` (`self.SM_Speaker_01_Holder_01`) (`KismetMathLibrary.MakeRotator` 0.0 0.0 (`self.Z (Yaw)`)) false false))
    (:`then_1`
      (`SplineComponent.SetLocationAtSplinePoint` (`self.Spline`) 0 (`SceneComponent.GetSocketLocation` (`self.SM_Speaker_01_Holder_02`) "Cable Wall") "World" true)
      (`SplineComponent.SetLocationAtSplinePoint` (`self.Spline`) 1 (`SceneComponent.GetSocketLocation` (`self.SM_Speaker_01_Main_01`) "Cable Main") "World" true))
    (:`then_2`
      (bind _returnvalue (`AddComponent|NODE_AddSplineMeshComponent-1`))
      (`SplineMeshComponent.SetStartAndEnd` _returnvalue _location_2 _tangent_2 _location _tangent true))))