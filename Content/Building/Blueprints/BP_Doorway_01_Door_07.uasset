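; Interactable door Blueprint that swings open and closed on alternating Interact calls.
; A FlipFlop plays or reverses a Timeline that yaws the door up to -90 degrees, turning the doorknob only during forward playback.
; Two DoOnce nodes reset each other to alternate the handle sound on opening and the closing sound on closing, both played at world origin.
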(event `self.Interact`
  (`GameplayStatics.PlaySoundAtLocation` null (0.0 0.0 0.0) (struct) 1.0 1.0 0.0 null null null null)
  (`/Engine/EditorBlueprintResources/StandardMacros.FlipFlop`
    (:`A`
      (`|ExecutionSequence`
        (:`then_0`
          (`/Engine/EditorBlueprintResources/StandardMacros.DoOnce` false :!label _label
            (:`Completed`
              (`GameplayStatics.PlaySoundAtLocation` "/Game/Building/Blueprints/DoorHandle1.DoorHandle1" (0.0 0.0 0.0) (struct) 1.0 1.0 0.0 null null null null)
              (goto _label_3 :!via `Reset`))))
        (:`then_1`
          (bind (_direction _doormove _doorhandle) (`Timeline|Timeline` :!label _label_2)
            (:`Update`
              (`SceneComponent.K2_SetRelativeRotation` (`self.Door`) (`KismetMathLibrary.MakeRotator` 0.0 0.0 (* _doormove -90.0)) false false)
              (if (not (`TimelineComponent.IsReversing` (`self.Timeline`)))
                (`SceneComponent.K2_SetRelativeRotation` (`self.Doorknob`) (`KismetMathLibrary.MakeRotator` (`KismetMathLibrary.Lerp` 0.0 -40.0 _doorhandle) 0.0 180.0) false false)))))))
    (:`B`
      (`|ExecutionSequence`
        (:`then_0`
          (goto _label_2 :!via `Reverse`))
        (:`then_1`
          (`/Engine/EditorBlueprintResources/StandardMacros.DoOnce` false :!label _label_3
            (:`Completed`
              (`GameplayStatics.PlaySoundAtLocation` "/Game/Building/Audio/Door_Closing.Door_Closing" (0.0 0.0 0.0) (struct) 1.0 1.0 0.0 null null null null)
              (goto _label :!via `Reset`))))))))

(fn `UserConstructionScript`)