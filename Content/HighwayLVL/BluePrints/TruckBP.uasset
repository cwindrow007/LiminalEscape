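; Truck actor for the highway level that starts a timed move when a BaseCharacter overlaps its StartTruck trigger.
; BeginPlay spawns a flare emitter at the child actor and caches the level's SplinePathBP2.
; The overlap plays the MoveTruck timeline at a rate set by TimeToComplete.
; Spline following looks unfinished: SetActorTransform receives no computed transform, the distance and Lerp nodes are unused, and debug prints remain.
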(event `self.ReceiveBeginPlay`
  (`|ExecutionSequence`
    (:`then_1`
      (`|SpawnActorFromClass` "/Game/HighwayLVL/BluePrints/Flare/FlareEmitter_Blueprint.FlareEmitter_Blueprint_C" (`KismetMathLibrary.Conv_VectorToTransform` (`SceneComponent.K2_GetComponentLocation` (`self.ChildActor`))) "Undefined" "MultiplyWithRoot" null null))
    (:`then_2`
      (bind _returnvalue (`GameplayStatics.GetActorOfClass` "/Game/HighwayLVL/BluePrints/SplinePathBP2.SplinePathBP2_C"))
      (set `self.SplineREF2` _returnvalue))
    (:`then_3`
      (set `self.Finished?` false))
    (:`then_4`
      (set `self.Close` true))
    (:`then_5`
      (for _index (range 0)
        (bind _output_get (set `self.LocalCurrentIndex` _index))
        (set `self.LocalNextIndex` (+ _output_get 1))))))

(event `self.StartTruck.OnComponentBeginOverlap`
  (params (OverlappedComponent :type "PrimitiveComponent Object Reference") (OtherActor :type "Actor Object Reference") (OtherComp :type "PrimitiveComponent Object Reference") (OtherBodyIndex :type Integer) (bFromSweep :type Boolean) (SweepResult :type "HitResult Structure (by ref)"))
  (cast `/Game/Blueprints/BaseCharacter` OtherActor)
  (`|ExecutionSequence`
    (:`then_0`
      (if (`self.Close`)
        (`TimelineComponent.SetPlayRate` (`self.MoveTruck`) (/ 1.0 (`self.TimeToComplete`)))
        (bind (_direction _truckmove) (`Timeline|MoveTruck` :!label _label)
          (:`Update`
            (`self.K2_SetActorTransform` (`KismetMathLibrary.MakeTransform` (0.0 0.0 0.0)))
            (`KismetSystemLibrary.Delay` 120.0)
            (goto _label :!via `Stop`))
          (:`Finished`
            (`KismetSystemLibrary.PrintString` "finished")
            (set `self.Finished?` true)))))
    (:`then_1`
      (if (`self.Finished?`)
        (`KismetSystemLibrary.PrintString` "mama")))))

(fn `UserConstructionScript`)