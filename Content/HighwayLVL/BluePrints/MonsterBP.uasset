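; MonsterBP is a monster that travels along a spline path, killing the player through DeathPit on the character when its Death collision overlaps them.
; Overlapping HesComing finds the MonsterSpline actor and starts the MonsterMove timeline at a rate inverse to MonsterRate.
; The timeline drives location and rotation along the spline's length.
; An always-lit flare emitter touching Death halts the timeline, which resumes after a long delay.
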(event `self.Death.OnComponentBeginOverlap`
  (params (OverlappedComponent :type "PrimitiveComponent Object Reference") (OtherActor :type "Actor Object Reference") (OtherComp :type "PrimitiveComponent Object Reference") (OtherBodyIndex :type Integer) (bFromSweep :type Boolean) (SweepResult :type "HitResult Structure (by ref)"))
  (bind _monsterspline (`/Game/HighwayLVL/BluePrints/MonsterSpline.MonsterSpline` (`self.MonsterPath`)))
  (`|ExecutionSequence`
    (:`then_0`
      (bind _asbase_character (cast `/Game/Blueprints/BaseCharacter` OtherActor))
      (`/Game/Blueprints/BaseCharacter.DeathPit` _asbase_character))
    (:`then_1`
      (cast `/Game/HighwayLVL/BluePrints/Flare/FlareEmitterALWAYSLIT` OtherActor)
      (`self.StopMonster`)
      (`KismetSystemLibrary.Delay` 150.0)
      (bind (_direction _newtrack_0) (`Timeline|MonsterMove` :!label _label)
        (:`Update`
          (bind _returnvalue (`KismetMathLibrary.Lerp` 0.0 (`SplineComponent.GetSplineLength` (`/Game/HighwayLVL/BluePrints/MonsterSpline.MonsterSpline` (`self.MonsterPath`))) _newtrack_0))
          (`self.K2_SetActorTransform` (`KismetMathLibrary.MakeTransform` (`SplineComponent.GetLocationAtDistanceAlongSpline` _monsterspline _returnvalue "World") (`SplineComponent.GetRotationAtDistanceAlongSpline` _monsterspline _returnvalue "World"))))))))

(event `self.HesComing.OnComponentBeginOverlap`
  (params (OverlappedComponent :type "PrimitiveComponent Object Reference") (OtherActor :type "Actor Object Reference") (OtherComp :type "PrimitiveComponent Object Reference") (OtherBodyIndex :type Integer) (bFromSweep :type Boolean) (SweepResult :type "HitResult Structure (by ref)"))
  (bind _returnvalue (`GameplayStatics.GetActorOfClass` "/Game/HighwayLVL/BluePrints/MonsterSpline.MonsterSpline_C"))
  (set `self.MonsterPath` _returnvalue)
  (`self.MonsterSpeed`))

(event `MonsterSpeed`
  (`TimelineComponent.SetPlayRate` (`self.MonsterMove`) (/ 1.0 (`self.MonsterRate`)))
  (goto _label))

(event `StopMonster`
  (goto _label :!via `Stop`))

(fn `UserConstructionScript`)