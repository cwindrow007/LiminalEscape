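; A sealed flare emitter actor that the player picks up and lights.
; Pickup fires FLAREVENT to mark the flare as held and returns the actor itself.
; Interact, only while held, hides the cap and trigger meshes, activates the Niagara effect and marks the flare lit.
; A GOODBYE event destroys the actor.
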(event `FLAREVENT`
  (set `self.IsInHand?` true))

(event `self.Interact`
  (if (`self.IsInHand?`)
    (`SceneComponent.SetVisibility` (`self.FlareTOP`) false false)
    (`ActorComponent.Activate` (`self.NiagaraComponent`) false)
    (`SceneComponent.SetVisibility` (`self.Trigger`) false false)
    (set `self.IsLit?` true)))

(event `GOODBYE`
  (`self.K2_DestroyActor`))

(fn `Pickup`
  (returns (StaticMesh :type "StaticMesh Object Reference") (NewParam :type "Actor Object Reference"))
  (`self.FLAREVENT`)
  (return null self))

(fn `UserConstructionScript`)